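; Gate Blueprint that slides a door cube down out of the way to open and back up to close.
; BeginPlay caches the cube's world location as the start point.
; Open plays a timeline that lerps the cube 400 units below that point, and Close reverses the same timeline from its end.
; Reset snaps the cube straight back to the cached start location.
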(event Custom|Open
  (bind _doorstart (Variables|Default|GetDoorStart))
  (bind _newtrack_0 (Timeline|TimelineOpen PlayFromStart)
    (:Update
      (Transformation|SetWorldLocation (Variables|Default|GetCube) (Math|Vector|Lerp(Vector) _doorstart (- _doorstart "0, 0,400.000000") _newtrack_0) false false))))

(event Custom|Close
  (bind _doorstart (Variables|Default|GetDoorStart))
  (bind _newtrack_0 (Timeline|TimelineOpen ReverseFromEnd)
    (:Update
      (Transformation|SetWorldLocation (Variables|Default|GetCube) (Math|Vector|Lerp(Vector) _doorstart (- _doorstart "0, 0,400.000000") _newtrack_0) false false))))

(event Custom|Reset
  (Transformation|SetWorldLocation (Variables|Default|GetCube) (Variables|Default|GetDoorStart) false false))

(event EventBeginPlay
  (Variables|Default|SetDoorStart (Transformation|GetWorldLocation (Variables|Default|GetCube))))

(event EventActorBeginOverlap
  (params (OtherActor :type Actor%20Object%20Reference)))

(event EventTick
  (params (DeltaSeconds :type Float%20%28single-precision%29)))

(fn ConstructionScript)