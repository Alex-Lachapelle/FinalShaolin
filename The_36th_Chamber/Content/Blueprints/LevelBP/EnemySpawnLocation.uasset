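; Enemy spawn point actor that tracks whether it is available, based on overlapping pawns and visibility to nearby players.
; It stores its transform at BeginPlay and becomes unavailable when a MasterPawn overlaps it.
; CheckForPlayer sphere-traces for the desired object types, then line-traces on Camera to each hit, ignoring MasterPawns.
; A clear line to the hit clears Available, otherwise it sets it, so the last hit decides.
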(event Custom|CheckForPlayer
  (bind _returnvalue (Transformation|GetActorLocation))
  (bind _outactors (Actor|GetAllActorsOfClass "/Game/Blueprints/Pawns/MasterPawn.MasterPawn_C"))
  (bind _outhits (Collision|MultiSphereTraceForObjects _returnvalue (+ _returnvalue "0, 0,15.000000") (Variables|Default|GetPlayerDetectionRadius) (Variables|Default|GetDesiredObjects) false _outactors "ForDuration"))
  (bind _array_element (Utilities|Array|ForEachLoopwithBreak _outhits)
    (:LoopBody
      (bind (_outhit _returnvalue_2) (Collision|LineTraceByChannel (Transformation|GetActorLocation) (Transformation|GetActorLocation (.HitActor (Collision|BreakHitResult _array_element))) "TraceTypeQuery2" false _outactors "None"))
      (if _returnvalue_2
        (if (== (.HitActor (Collision|BreakHitResult _outhit)) (.HitActor (Collision|BreakHitResult _array_element)))
          (Variables|Default|SetAvailable false)
          (else
            (Variables|Default|SetAvailable true)))
        (else
          (Variables|Default|SetAvailable true))))))

(event EventBeginPlay
  (Variables|Default|SetCurrentTransform (Transformation|GetActorTransform)))

(event EventActorBeginOverlap
  (params (OtherActor :type Actor%20Object%20Reference)))

(event EventTick
  (params (DeltaSeconds :type Float%20%28single-precision%29)))

(event Collision|EventActorBeginOverlap
  (params (OtherActor :type Actor%20Object%20Reference))
  (bind _asmaster_pawn (Utilities|Casting|CastToMasterPawn OtherActor))
  (if (== OtherActor _asmaster_pawn)
    (Variables|Default|SetAvailable false)))

(fn ConstructionScript)