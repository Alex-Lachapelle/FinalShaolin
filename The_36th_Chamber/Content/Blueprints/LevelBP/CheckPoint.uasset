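; Checkpoint trigger actor that moves the level's player spawn to a new location when the player reaches it.
; On BeginPlay it caches the transform of its attached spawnpoint.
; The first overlap by player pawn 0, gated by a DoOnce, teleports the first PlayerSpawn actor found to that transform.
; The construction script sizes the trigger box from the BoxSize variable.
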(event EventBeginPlay
  (Variables|Default|SetCheckpointTransform (Transformation|GetActorTransform (Variables|Default|GetAttachedSpawnpoint))))

(event EventActorBeginOverlap
  (params (OtherActor :type Actor%20Object%20Reference))
  (bind _checkpointtransform (Variables|Default|GetCheckpointTransform))
  (bind (_location _rotation) (Math|Transform|BreakTransform _checkpointtransform))
  (if (== OtherActor (Game|Player|GetPlayerPawn 0))
    (Utilities|FlowControl|DoOnce false
      (:Completed
        (bind _outactors (Actor|GetAllActorsOfClass "/Game/Blueprints/LevelBP/PlayerSpawn.PlayerSpawn_C"))
        (Transformation|Teleport (Utilities|Array|Get(acopy) _outactors) _location _rotation)))))

(event EventTick
  (params (DeltaSeconds :type Float%20%28single-precision%29)))

(fn ConstructionScript
  (Variables|Default|SetAttachedSpawnpoint (Variables|Default|GetAttachedSpawnpoint))
  (Components|Box|SetBoxExtent (Variables|Default|GetBox) (Variables|Default|GetBoxSize) true))