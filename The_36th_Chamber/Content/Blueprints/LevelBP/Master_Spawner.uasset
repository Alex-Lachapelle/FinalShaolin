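; Master spawner actor that spawns waves of enemies at its attached EnemySpawnLocation points and signals when a wave is cleared.
; SpawnWave staggers spawns through a delayed-loop macro, using Check to pick the available point nearest the player.
; It binds each MasterPawn's death to BotDead, which counts down to CallWaveCleared.
; ManualSpawn instead splits enemies between the first two undestroyed points, without binding death.
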(event Custom|ManualSpawn
  (params (NumberOfEnemies :type Integer) (EnemyType :type Actor%20Class%20Reference) (SpawnIndex :type Integer))
  (bind _attachedspawns (Variables|Default|GetAttachedSpawns))
  (bind _attachedspawns_2 (Variables|Default|GetAttachedSpawns))
  (bind _item (Utilities|Array|Get(acopy) _attachedspawns 1))
  (bind _item_2 (Utilities|Array|Get(acopy) _attachedspawns_2))
  (bind _asenemy_spawn_location (Utilities|Casting|CastToEnemySpawnLocation _item))
  (bind _asenemy_spawn_location_2 (Utilities|Casting|CastToEnemySpawnLocation _item_2))
  ;[1 1 1] Manual Spawn
  (bind _index (Utilities|ForLoopDelay 1 NumberOfEnemies 0.5)
    (:LoopBody
      (if (Variables|Default|GetSpawn?)
        (if (> _index (/ NumberOfEnemies 2))
          (if (not (Variables|/Game/Blueprints/LevelBP/EnemySpawnLocation.EnemySpawnLocation_C|GetDestroyed? _asenemy_spawn_location))
            (bind _returnvalue (Game|SpawnActorfromClass EnemyType (Variables|/Game/Blueprints/LevelBP/EnemySpawnLocation.EnemySpawnLocation_C|GetCurrentTransform _asenemy_spawn_location) "AdjustIfPossibleButAlwaysSpawn" 0 0))
            (Variables|Default|SetSpawnedPawn _returnvalue)
            (Variables|Default|SetSpawnCounter (+ (Variables|Default|GetSpawnCounter) 1))
            (Utilities|Casting|CastToMasterPawn (Variables|Default|GetSpawnedPawn)))
          (elif (not (Variables|/Game/Blueprints/LevelBP/EnemySpawnLocation.EnemySpawnLocation_C|GetDestroyed? _asenemy_spawn_location_2))
            (bind _returnvalue_2 (Game|SpawnActorfromClass EnemyType (Variables|/Game/Blueprints/LevelBP/EnemySpawnLocation.EnemySpawnLocation_C|GetCurrentTransform _asenemy_spawn_location_2) "AdjustIfPossibleButAlwaysSpawn" 0 0))
            (Variables|Default|SetSpawnedPawn _returnvalue_2)
            (Variables|Default|SetSpawnCounter (+ (Variables|Default|GetSpawnCounter) 1))
            (Utilities|Casting|CastToMasterPawn (Variables|Default|GetSpawnedPawn))))))))

(event Custom|SpawnWave
  (params (Number%20Of%20Enemies :type Integer) (EnemyType :type Actor%20Class%20Reference))
  ;[1 1 1] Auto Spawn Enemies
  (Utilities|ForLoopDelay 1 Number%20Of%20Enemies 0.5
    (:LoopBody
      (if (Variables|Default|GetSpawn?)
        (CallFunction|Check)
        (bind _returnvalue (Game|SpawnActorfromClass EnemyType (Variables|Default|GetSpawnTransform) "AdjustIfPossibleButAlwaysSpawn" 0 0))
        (Variables|Default|SetSpawnedPawn _returnvalue)
        (Variables|Default|SetSpawnCounter (+ (Variables|Default|GetSpawnCounter) 1))
        (bind _asmaster_pawn (Utilities|Casting|CastToMasterPawn (Variables|Default|GetSpawnedPawn)))
        (EventDispatchers|BindEventtoDeath _asmaster_pawn (delegate Custom|BotDead))))))

(event Custom|Check
  ;[1 1 1] Check For Player Location
  (for _index (range 0 (Utilities|Array|Length (Variables|Default|GetAttachedSpawns)))
    (bind _asenemy_spawn_location (Utilities|Casting|CastToEnemySpawnLocation (Utilities|Array|Get(acopy) (Variables|Default|GetAttachedSpawns) _index)))
    (Default|CheckforPlayer _asenemy_spawn_location)
    (if (Variables|/Game/Blueprints/LevelBP/EnemySpawnLocation.EnemySpawnLocation_C|GetAvailable _asenemy_spawn_location)
      (bind _asenemy_spawn_location_2 (Utilities|Casting|CastToEnemySpawnLocation (Utilities|Array|Get(acopy) (Variables|Default|GetAttachedSpawns) _index)))
      (Utilities|Array|Insert (Variables|Default|GetAvailableSpawns) _asenemy_spawn_location_2 (Variables|Default|GetCounter))
      (Variables|Default|SetCounter (+ (Variables|Default|GetCounter) 1))
      (for (_array_element _array_index) (Variables|Default|GetAvailableSpawns)
        (Math|Float|CompareFloat (Transformation|GetDistanceTo _array_element (Game|Player|GetPlayerPawn 0)) (Variables|Default|GetCurrentShortestDistance)
          (:<
            (Variables|Default|SetCurrentShortestDistance (Transformation|GetDistanceTo _array_element (Game|Player|GetPlayerPawn 0)))
            (Variables|Default|SetCurrentIndex _array_index))))
      (Variables|Default|SetSpawnTransform (Variables|/Game/Blueprints/LevelBP/EnemySpawnLocation.EnemySpawnLocation_C|GetCurrentTransform (Utilities|Array|Get(acopy) (Variables|Default|GetAvailableSpawns) (Variables|Default|GetCurrentIndex))))
      (Variables|Default|SetCounter 0)
      (Variables|Default|SetCurrentIndex 0)
      (else
        (bind _asenemy_spawn_location_3 (Utilities|Casting|CastToEnemySpawnLocation (Utilities|Array|Get(acopy) (Variables|Default|GetAttachedSpawns) _index)))
        (Utilities|Array|RemoveItem (Variables|Default|GetAvailableSpawns) _asenemy_spawn_location_3))))
  (Variables|Default|SetCounter 0))

(event Custom|BotDead
  ;[1 1 1] Auto Spawn Enemies
  (Variables|Default|SetSpawnCounter (- (Variables|Default|GetSpawnCounter) 1))
  (if (== (Variables|Default|GetSpawnCounter) 0)
    (Default|CallWaveCleared)
    (else
      (Utilities|FlowControl|Delay 5.0))))

(event EventBeginPlay
  (Rendering|SetVisibility (Variables|Default|GetCube) false false))

(event EventActorBeginOverlap
  (params (OtherActor :type Actor%20Object%20Reference)))

(event EventTick
  (params (DeltaSeconds :type Float%20%28single-precision%29)))

(fn ConstructionScript
  (Variables|Default|SetAttachedSpawns (Variables|Default|GetAttachedSpawns)))

(fn StopSpawn
  (Variables|Default|SetSpawn? true))

(fn Spawn
  (params (Number%20of%20Enemies :type Integer) (EnemyType :type Actor%20Class%20Reference))
  (bind _counter (Utilities|FlowControl|DoN Number%20of%20Enemies :!label _label)
    (:Exit
      (CallFunction|Check)
      (if (Variables|Default|GetSpawn?)
        (Variables|Default|SetSpawn? false)
        (Game|SpawnActorfromClass EnemyType (Variables|Default|GetSpawnTransform) "Undefined" 0 0)
        (if (== _counter Number%20of%20Enemies)
          (goto _label Reset)
          (else
            (Utilities|Time|SetTimerbyFunctionName 0 "StopSpawn" 1.0)
            (return Number%20of%20Enemies)))))))