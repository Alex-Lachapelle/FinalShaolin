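; Save game Blueprint that holds player display settings and a save slot name.
; Stored settings include gamma, field of view, post-process quality, fullscreen state and a resolution enum.
; A Callout event prints each stored value to the screen for debugging.
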(event Custom|Callout
  (Development|PrintString 0 (Variables|Default|GetSaveSlotName))
  (Development|PrintString 0 (Utilities|String|ToString(Float) (Variables|Settings|GetGamma)))
  (Development|PrintString 0 (Utilities|String|ToString(Float) (Variables|Settings|GetFieldOfView)))
  (Development|PrintString 0 (Utilities|String|ToString(Integer) (Variables|Settings|GetPostProcessQuality)))
  (Development|PrintString 0 (Utilities|String|ToString(Boolean) (Variables|Settings|GetFullscreen)))
  (Development|PrintString 0 (Utilities|String|EnumtoString (Variables|Settings|GetResolutions))))