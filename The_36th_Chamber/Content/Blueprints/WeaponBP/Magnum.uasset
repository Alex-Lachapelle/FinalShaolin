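; Magnum weapon Blueprint that fires small projectiles and remotely detonates them with alt fire.
; Main fire spawns and saves each Magnum_Proj, spends ammo and uses a timer for fire rate or, on the last round, reload delay with an immediate counter refill.
; Alt fire steps through the saved projectiles by a persistent index, calling Detonate on each with a short delay between them.
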(event EventFireAlt
  (if (== (Utilities|Array|Length (Variables|Default|GetSavedProjectile)) 0) :!label _label
    (Variables|Default|SetMagnumIndex 0)
    (else
      (bind _asmagnum_proj (Utilities|Casting|CastToMagnum_Proj (Utilities|Array|Get(acopy) (Variables|Default|GetSavedProjectile) (Variables|Default|GetMagnumIndex))))
      (Default|Detonate _asmagnum_proj)
      (Variables|Default|SetMagnumIndex (+ (Variables|Default|GetMagnumIndex) 1))
      (Utilities|FlowControl|Delay 0.2)
      (goto _label))))

(event EventBeginPlay
  (|CallParentFunction)
  (bind _output_get (Variables|Default|SetPistolAmmo (Variables|Default|GetMaxPistolAmmo)))
  (CallFunction|Switched _output_get))

(event EventActorBeginOverlap
  (params (OtherActor :type Actor%20Object%20Reference)))

(event EventTick
  (params (DeltaSeconds :type Float%20%28single-precision%29)))

(event EventFireMain
  (|CallParentFunction)
  (if (Variables|Default|GetCanFire?)
    (Variables|Default|SetCanFire? false)
    (if (> (Variables|Default|GetPistolAmmo) 0)
      (bind _returnvalue (Game|SpawnActorfromClass "/Game/Blueprints/WeaponBP/Magnum_Proj.Magnum_Proj_C" (Variables|Default|GetProjectileHit) "AdjustIfPossibleButDontSpawnIfColliding" 0 "0.100000,0.100000,0.100000" 0)) ; Spawn projectile
      (Utilities|Array|Add (Variables|Default|GetSavedProjectile) _returnvalue)
      (bind _output_get (Variables|Default|SetPistolAmmo (- (Variables|Default|GetPistolAmmo) 1)))
      (CallFunction|UpdateAmmo _output_get)
      (if (> (Variables|Default|GetPistolAmmo) 0)
        (Utilities|Time|SetTimerbyFunctionName 0 "ShotTimerExpired" (Variables|Default|GetPistolFireRate))
        (Audio|PlaySoundatLocation "/Game/ArtAssets/Audio/FirstPersonTemplateWeaponFire02.FirstPersonTemplateWeaponFire02" (Transformation|GetActorLocation)) ; Play firing sound
        (else
          (Utilities|Time|SetTimerbyFunctionName 0 "ShotTimerExpired" (Variables|Default|GetPistolReloadTime))
          (Variables|Default|SetPistolAmmo (Variables|Default|GetMaxPistolAmmo)))))))

(fn ConstructionScript
  (|CallParentFunction))