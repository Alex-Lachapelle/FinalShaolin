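; Base weapon Blueprint, apparently a parent for specific guns, with empty hooks for alt fire and trigger releases.
; FireMain line-traces from the first-person camera to MaxRange, then stores a ProjectileHit transform at the character's GunTransform location, aimed at the impact or max-range point.
; It only computes aim; nothing here spawns projectiles or spends ammo.
; Switched sets max and current ammo from the passed value, and ShotTimerExpired re-enables CanFire.
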(event Custom|Switched
  (params (WeaponAmmo :type Integer))
  (bind _output_get (Variables|Default|SetCurrentMaxAmmo WeaponAmmo))
  (CallFunction|UpdateAmmo _output_get))

(event Custom|FireMain
  (bind _asfirst_person_character (Utilities|Casting|CastToFirstPersonCharacter (Game|Player|GetPlayerPawn 0)))
  (Variables|Default|SetMaxRangeHitPoint (+ (Transformation|GetWorldLocation (Variables|/Game/Blueprints/FirstPersonCharacter.FirstPersonCharacter_C|GetFirstPersonCamera _asfirst_person_character)) (* (Math|Vector|GetForwardVector (Transformation|GetWorldRotation (Variables|/Game/Blueprints/FirstPersonCharacter.FirstPersonCharacter_C|GetFirstPersonCamera _asfirst_person_character))) (Variables|Default|GetMaxRange))))
  (bind (_outhit _returnvalue) (Collision|LineTraceByChannel (Transformation|GetWorldLocation (Variables|/Game/Blueprints/FirstPersonCharacter.FirstPersonCharacter_C|GetFirstPersonCamera _asfirst_person_character)) (+ (Transformation|GetWorldLocation (Variables|/Game/Blueprints/FirstPersonCharacter.FirstPersonCharacter_C|GetFirstPersonCamera _asfirst_person_character)) (* (Math|Vector|GetForwardVector (Transformation|GetWorldRotation (Variables|/Game/Blueprints/FirstPersonCharacter.FirstPersonCharacter_C|GetFirstPersonCamera _asfirst_person_character))) (Variables|Default|GetMaxRange))) "TraceTypeQuery1" true 0 "None"))
  (Variables|Default|SetHitResult _outhit)
  (Variables|Default|SetImpactPoint (.ImpactPoint (Collision|BreakHitResult _outhit)))
  (bind _asfirst_person_character_2 (Utilities|Casting|CastToFirstPersonCharacter (Game|Player|GetPlayerPawn 0))
    (:then
      _)
    (:CastFailed
      _))
  (if _returnvalue
    (Variables|Default|SetProjectileHit (Math|Transform|MakeTransform (.Location (Math|Transform|BreakTransform (Variables|/Game/Blueprints/FirstPersonCharacter.FirstPersonCharacter_C|GetGunTransform _asfirst_person_character_2))) (Math|Rotator|MakeRotfromX (- (.ImpactPoint (Collision|BreakHitResult _outhit)) (.Location (Math|Transform|BreakTransform (Variables|/Game/Blueprints/FirstPersonCharacter.FirstPersonCharacter_C|GetGunTransform _asfirst_person_character_2)))))))
    (else
      (Variables|Default|SetProjectileHit (Math|Transform|MakeTransform (.Location (Math|Transform|BreakTransform (Variables|/Game/Blueprints/FirstPersonCharacter.FirstPersonCharacter_C|GetGunTransform _asfirst_person_character_2))) (Math|Rotator|MakeRotfromX (- (Variables|Default|GetMaxRangeHitPoint) (.Location (Math|Transform|BreakTransform (Variables|/Game/Blueprints/FirstPersonCharacter.FirstPersonCharacter_C|GetGunTransform _asfirst_person_character_2))))))))))

(event Custom|FireAlt)

(event Custom|UpdateAmmo
  (params (Current%20Ammo :type Integer))
  (Variables|Default|SetCurrentAmmo Current%20Ammo))

(event Custom|MainRelease)

(event Custom|AltRelease)

(event EventBeginPlay)

(event EventTick
  (params (DeltaSeconds :type Float%20%28single-precision%29)))

(fn ConstructionScript)

(fn ShotTimerExpired
  (Variables|Default|SetCanFire? true))