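; Railgun weapon Blueprint that extends a parent weapon with a rate-limited primary fire and a zoom alt-fire.
; FireMain calls the parent, then, if CanFire is set, clears it, starts a ShotTimerExpired timer using RailgunFireRate, and plays the firing sound.
; FireAlt and AltRelease call Zoom and UnZoom on player 0's FirstPersonCharacter.
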(event EventFireMain
  (|CallParentFunction)
  (if (Variables|Default|GetCanFire?)
    (Variables|Default|SetCanFire? false)
    (Utilities|Time|SetTimerbyFunctionName 0 "ShotTimerExpired" (Variables|Default|GetRailgunFireRate))
    (Audio|PlaySoundatLocation "/Game/ArtAssets/Audio/FirstPersonTemplateWeaponFire02.FirstPersonTemplateWeaponFire02" (Transformation|GetActorLocation)) ; Play firing sound
  ))

(event EventBeginPlay
  (|CallParentFunction))

(event EventFireAlt
  (bind _asfirst_person_character (Utilities|Casting|CastToFirstPersonCharacter (Game|Player|GetPlayerPawn 0)))
  (Default|Zoom _asfirst_person_character))

(event EventActorBeginOverlap
  (params (OtherActor :type Actor%20Object%20Reference)))

(event EventTick
  (params (DeltaSeconds :type Float%20%28single-precision%29)))

(event EventAltRelease
  (bind _asfirst_person_character (Utilities|Casting|CastToFirstPersonCharacter (Game|Player|GetPlayerPawn 0)))
  (Default|UnZoom _asfirst_person_character))

(fn ConstructionScript
  (|CallParentFunction))