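; Shotgun projectile child class that scales damage by range and expires through a short max lifetime or impacts.
; On overlap it divides Damage by the target's distance from player pawn 0 before calling parent logic, and prints that distance factor.
; Hits on a MasterPawn destroy it, while other hits count bounces until the second destroys it.
; The gravity increase sits behind the successful pawn cast, so ordinary bounces never reach it.
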(event EventBeginPlay
  (CallFunction|SetDamage (Variables|Default|GetDamage))
  (|CallParentFunction)
  (Variables|Default|SetMaxLifetime 4.0))

(event EventActorBeginOverlap
  (params (OtherActor :type Actor%20Object%20Reference))
  (Variables|Default|SetHitLocation (Transformation|GetActorLocation OtherActor))
  (CallFunction|SetDamage (/ (Variables|Default|GetDamage) (/ (Math|Vector|VectorLength (- (Variables|Default|GetHitLocation) (Transformation|GetActorLocation (Game|Player|GetPlayerPawn 0)))) 6e+01)))
  (|CallParentFunction OtherActor)
  (Development|PrintString (Utilities|String|ToString(Integer) (Math|Float|Truncate (/ (Math|Vector|VectorLength (- (Variables|Default|GetHitLocation) (Transformation|GetActorLocation (Game|Player|GetPlayerPawn 0)))) 6e+01)))))

(event EventTick
  (params (DeltaSeconds :type Float%20%28single-precision%29)))

(event Collision|EventHit
  (params (MyComp :type Primitive%20Component%20Object%20Reference) (Other :type Actor%20Object%20Reference) (OtherComp :type Primitive%20Component%20Object%20Reference) (bSelfMoved :type Boolean) (HitLocation :type Vector) (HitNormal :type Vector :default "0, 0, 0") (NormalImpulse :type Vector :default "0, 0, 0") (Hit :type Hit%20Result%20Structure%20%28by%20ref%29))
  (Utilities|FlowControl|Sequence
    (:then_0
      (bind _asmaster_pawn (Utilities|Casting|CastToMasterPawn Other))
      (if (== _asmaster_pawn Other)
        (Actor|DestroyActor :!label _label)
        (else
          (Variables|/Script/Engine.ProjectileMovementComponent|SetProjectileGravityScale (Variables|Default|GetProjectile) 1.2)
          (if (== (Variables|Default|GetBounces) 2) :!label _label_2
            (goto _label)))))
    (:then_1
      (Variables|Default|SetBounces (+ (Variables|Default|GetBounces) 1))
      (goto _label_2))))

(fn ConstructionScript
  (|CallParentFunction))