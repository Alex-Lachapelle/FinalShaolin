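; GrenadeLauncher is a child weapon Blueprint that fires grenade projectiles.
; It overrides FireMain, calls the parent, then, if CanFire is set, clears that flag and spawns a scaled-down Grenade_Proj at the ProjectileHit transform.
; A FireRate timer then calls ShotTimerExpired by name, a function not defined in this Blueprint, to pace shots.
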(event EventBeginPlay
  (|CallParentFunction))

(event EventActorBeginOverlap
  (params (OtherActor :type Actor%20Object%20Reference)))

(event EventTick
  (params (DeltaSeconds :type Float%20%28single-precision%29))
  (|CallParentFunction 0.0))

(event EventFireMain
  (|CallParentFunction)
  (if (Variables|Default|GetCanFire?)
    (Variables|Default|SetCanFire? false)
    (Game|SpawnActorfromClass "/Game/Blueprints/WeaponBP/Grenade_Proj.Grenade_Proj_C" (Variables|Default|GetProjectileHit) "AdjustIfPossibleButDontSpawnIfColliding" 0 "0.100000,0.100000,0.100000" 0) ; Spawn projectile
    (Utilities|Time|SetTimerbyFunctionName 0 "ShotTimerExpired" (Variables|Default|GetFireRate))))

(fn ConstructionScript
  (|CallParentFunction))