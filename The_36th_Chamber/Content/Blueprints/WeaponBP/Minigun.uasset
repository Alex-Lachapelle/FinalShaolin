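; Minigun weapon Blueprint that fires spread projectiles continuously while the fire input is held.
; FireMain and MainRelease open and close a Tick gate, which line-traces from the player camera to aim shots from the gun transform at the crosshair target.
; Timers calling ShotTimerExpired pace fire rate and reload, with ammo refilling as the reload starts.
; Releasing fire immediately re-enables CanFire, even mid-cooldown or reload.
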(event EventBeginPlay
  (|CallParentFunction)
  (bind _output_get (Variables|Default|SetMinigunAmmo (Variables|Default|GetMaxMinigunAmmo)))
  (CallFunction|Switched _output_get))

(event EventActorBeginOverlap
  (params (OtherActor :type Actor%20Object%20Reference)))

(event EventTick
  (params (DeltaSeconds :type Float%20%28single-precision%29))
  (Utilities|FlowControl|Gate true
    (:Exit
      (bind _asfirst_person_character (Utilities|Casting|CastToFirstPersonCharacter (Game|Player|GetPlayerPawn 0)))
      (Variables|Default|SetMaxRangeHitPoint (+ (Transformation|GetWorldLocation (Variables|/Game/Blueprints/Player/FirstPersonCharacter.FirstPersonCharacter_C|GetFirstPersonCamera _asfirst_person_character)) (* (Math|Vector|GetForwardVector (Transformation|GetWorldRotation (Variables|/Game/Blueprints/Player/FirstPersonCharacter.FirstPersonCharacter_C|GetFirstPersonCamera _asfirst_person_character))) (Variables|Default|GetMaxRange))))
      (bind (_outhit _returnvalue) (Collision|LineTraceByChannel (Transformation|GetWorldLocation (Variables|/Game/Blueprints/Player/FirstPersonCharacter.FirstPersonCharacter_C|GetFirstPersonCamera _asfirst_person_character)) (+ (Transformation|GetWorldLocation (Variables|/Game/Blueprints/Player/FirstPersonCharacter.FirstPersonCharacter_C|GetFirstPersonCamera _asfirst_person_character)) (* (Math|Vector|GetForwardVector (Transformation|GetWorldRotation (Variables|/Game/Blueprints/Player/FirstPersonCharacter.FirstPersonCharacter_C|GetFirstPersonCamera _asfirst_person_character))) (Variables|Default|GetMaxRange))) "TraceTypeQuery1" false 0 "None"))
      (bind _asfirst_person_character_2 (Utilities|Casting|CastToFirstPersonCharacter (Game|Player|GetPlayerPawn 0))
        (:then
          _)
        (:CastFailed
          _))
      (Default|GetGunTransform _asfirst_person_character_2)
      (if _returnvalue
        (Variables|Default|SetMinigunHit (Math|Transform|MakeTransform (.Location (Math|Transform|BreakTransform (Variables|/Game/Blueprints/Player/FirstPersonCharacter.FirstPersonCharacter_C|GetGunTransform _asfirst_person_character_2))) (Math|Rotator|MakeRotfromX (- (.ImpactPoint (Collision|BreakHitResult _outhit)) (.Location (Math|Transform|BreakTransform (Variables|/Game/Blueprints/Player/FirstPersonCharacter.FirstPersonCharacter_C|GetGunTransform _asfirst_person_character_2)))))))
        (else
          (Variables|Default|SetMinigunHit (Math|Transform|MakeTransform (.Location (Math|Transform|BreakTransform (Variables|/Game/Blueprints/Player/FirstPersonCharacter.FirstPersonCharacter_C|GetGunTransform _asfirst_person_character_2))) (Math|Rotator|MakeRotfromX (- (Variables|Default|GetMaxRangeHitPoint) (.Location (Math|Transform|BreakTransform (Variables|/Game/Blueprints/Player/FirstPersonCharacter.FirstPersonCharacter_C|GetGunTransform _asfirst_person_character_2)))))))))
      (Variables|Default|SetReleased? false)
      (if (Variables|Default|GetCanFire?)
        (if (not (Variables|Default|GetReleased?))
          (Game|SpawnActorfromClass "/Game/Blueprints/WeaponBP/Master_Projectile.Master_Projectile_C" (Math|Transform|MakeTransform (.Location (Math|Transform|BreakTransform (Variables|Default|GetMinigunHit))) (Math|Rotator|MakeRotfromX (+ (+ (.X (Math|Rotator|GetAxes (.Rotation (Math|Transform|BreakTransform (Variables|Default|GetMinigunHit))))) (* (.Y (Math|Rotator|GetAxes (.Rotation (Math|Transform|BreakTransform (Variables|Default|GetMinigunHit))))) (Math|Random|RandomFloatinRange -0.02 0.02))) (* (.Z (Math|Rotator|GetAxes (.Rotation (Math|Transform|BreakTransform (Variables|Default|GetMinigunHit))))) (Math|Random|RandomFloatinRange -0.02 0.02))))) "AdjustIfPossibleButDontSpawnIfColliding" 0 "0.000000,0.000000,0.000000" 0) ; Spawn projectile
          (Variables|Default|SetCanFire? false)
          (bind _output_get (Variables|Default|SetMinigunAmmo (- (Variables|Default|GetMinigunAmmo) 1)))
          (CallFunction|UpdateAmmo _output_get)
          (if (> (Variables|Default|GetMinigunAmmo) 0)
            (Utilities|Time|SetTimerbyFunctionName 0 "ShotTimerExpired" (Variables|Default|GetMinigunFirerate))
            (Audio|PlaySoundatLocation "/Game/ArtAssets/Audio/FirstPersonTemplateWeaponFire02.FirstPersonTemplateWeaponFire02" (Transformation|GetActorLocation)) ; Play firing sound
            (else
              (Utilities|Time|SetTimerbyFunctionName 0 "ShotTimerExpired" (Variables|Default|GetMinigunReloadTime))
              (Variables|Default|SetMinigunAmmo (Variables|Default|GetMaxMinigunAmmo)))))))))

(event EventFireMain
  (Utilities|FlowControl|Gate true) ; enters at Open
)

(event EventMainRelease
  (Variables|Default|SetReleased? true)
  (Variables|Default|SetCanFire? true)
  (Utilities|FlowControl|Gate true) ; enters at Close
)

(fn ConstructionScript
  (|CallParentFunction))