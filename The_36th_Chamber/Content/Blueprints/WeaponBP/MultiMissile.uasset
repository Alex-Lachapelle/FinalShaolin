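; MultiMissile is a child weapon Blueprint that fires a volley of MM_Proj missiles on primary fire.
; FireMain spawns BulletAmount projectiles, passing itself as ParentGun, then blocks firing until the ShotTimerExpired timer runs at the fire rate.
; Each spawn transform comes from a Transform helper, whose sine and cosine math spaces shots evenly around a Spread-sized ring on the ProjectileHit aim axes.
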(event EventTick
  (params (DeltaSeconds :type Float%20%28single-precision%29))
  (|CallParentFunction)
  (bind _asfirst_person_character (Utilities|Casting|CastToFirstPersonCharacter (Game|Player|GetPlayerPawn 0)))
  (Default|GetGunTransform _asfirst_person_character))

(event EventMainRelease)

(event EventBeginPlay
  (|CallParentFunction))

(event EventActorBeginOverlap
  (params (OtherActor :type Actor%20Object%20Reference)))

(event EventTick
  (params (DeltaSeconds :type Float%20%28single-precision%29))
  (|CallParentFunction 0.0))

(event EventFireMain
  (bind _bulletamount (Variables|Default|GetBulletAmount))
  ;[1 1 1] Outer Radius
  (if (Variables|Default|GetCanFire?)
    (Variables|Default|SetCanFire? false)
    (for _index (range 1 _bulletamount)
      (Game|SpawnActorfromClass "/Game/Blueprints/WeaponBP/MM_Proj.MM_Proj_C" (Utilities|Transform (Variables|Default|GetSpread) _index _bulletamount) "AdjustIfPossibleButDontSpawnIfColliding" 0 self "0.000000,0.000000,0.000000") ; Spawn projectile
    )
    (Utilities|Time|SetTimerbyFunctionName 0 "ShotTimerExpired" (Variables|Default|GetFirerate))))

(fn ConstructionScript
  (|CallParentFunction))