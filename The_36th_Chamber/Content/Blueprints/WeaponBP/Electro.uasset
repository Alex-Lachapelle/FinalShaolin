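; Electro weapon Blueprint that shows a continuous particle beam from the player's gun while primary fire is held.
; FireMain opens a gate on Tick and MainRelease closes it and deactivates the particle system, with CanFire tracking the held state.
; Each gated tick line traces forward from the first-person character's gun transform and sets the beam endpoints to the muzzle and the impact point or maximum range.
; It applies no damage.
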(event EventBeginPlay
  (|CallParentFunction))

(event EventActorBeginOverlap
  (params (OtherActor :type Actor%20Object%20Reference)))

(event EventTick
  (params (DeltaSeconds :type Float%20%28single-precision%29))
  (bind _particlesystem (Variables|Default|GetParticleSystem))
  (Utilities|FlowControl|Gate true
    (:Exit
      (Components|Activation|Activate (Variables|Default|GetParticleSystem) false)
      (bind _asfirst_person_character (Utilities|Casting|CastToFirstPersonCharacter (Game|Player|GetPlayerPawn 0)))
      (Default|GetGunTransform _asfirst_person_character)
      (bind (_outhit _returnvalue) (Collision|LineTraceByChannel (.Location (Math|Transform|BreakTransform (Variables|/Game/Blueprints/FirstPersonCharacter.FirstPersonCharacter_C|GetGunTransform _asfirst_person_character))) (+ (.Location (Math|Transform|BreakTransform (Variables|/Game/Blueprints/FirstPersonCharacter.FirstPersonCharacter_C|GetGunTransform _asfirst_person_character))) (* (Math|Vector|GetForwardVector (.Rotation (Math|Transform|BreakTransform (Variables|/Game/Blueprints/FirstPersonCharacter.FirstPersonCharacter_C|GetGunTransform _asfirst_person_character)))) 1.5e+03)) "TraceTypeQuery1" true 0 "None"))
      (if (not (Variables|Default|GetCanFire?))
        (Class|ParticleSystemComponent|SetBeamSourcePoint _particlesystem 0 (.Location (Math|Transform|BreakTransform (Variables|/Game/Blueprints/FirstPersonCharacter.FirstPersonCharacter_C|GetGunTransform _asfirst_person_character))))
        (if _returnvalue
          (Class|ParticleSystemComponent|SetBeamTargetPoint _particlesystem 0 (.ImpactPoint (Collision|BreakHitResult _outhit)))
          (else
            (Class|ParticleSystemComponent|SetBeamTargetPoint _particlesystem 0 (+ (.Location (Math|Transform|BreakTransform (Variables|/Game/Blueprints/FirstPersonCharacter.FirstPersonCharacter_C|GetGunTransform _asfirst_person_character))) (* (Math|Vector|GetForwardVector (.Rotation (Math|Transform|BreakTransform (Variables|/Game/Blueprints/FirstPersonCharacter.FirstPersonCharacter_C|GetGunTransform _asfirst_person_character)))) 1.5e+03)))))))))

(event EventFireMain
  (bind _particlesystem (Variables|Default|GetParticleSystem))
  (if (Variables|Default|GetCanFire?)
    (Variables|Default|SetCanFire? false)
    (Utilities|FlowControl|Gate true) ; enters at Open
  ))

(event EventMainRelease
  (bind _particlesystem (Variables|Default|GetParticleSystem))
  (bind _particlesystem_2 (Variables|Default|GetParticleSystem))
  (Variables|Default|SetCanFire? true)
  (Utilities|FlowControl|Sequence
    (:then_0
      (Utilities|FlowControl|Gate true) ; enters at Close
    )
    (:then_1
      (Components|Activation|Deactivate _particlesystem_2))))

(fn ConstructionScript
  (|CallParentFunction))