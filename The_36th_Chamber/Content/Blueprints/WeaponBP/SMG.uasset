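; SMG weapon Blueprint that fires automatically while the trigger is held, then detonates its projectiles on release.
; A Tick-driven gate, opened by FireMain, spawns SMG_Proj actors into a saved array, spending ammo and using ShotTimerExpired timers for fire rate and reload.
; MainRelease closes the gate and, after a short delay, steps through the saved projectiles, detonating them one by one in a delayed loop.
; Alt fire is empty.
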(event EventFireAlt)

(event EventBeginPlay
  (|CallParentFunction)
  (bind _output_get (Variables|Default|SetPistolAmmo (Variables|Default|GetMaxPistolAmmo)))
  (CallFunction|Switched _output_get))

(event Collision|EventActorBeginOverlap
  (params (OtherActor :type Actor%20Object%20Reference)))

(event EventTick
  (params (DeltaSeconds :type Float%20%28single-precision%29))
  (Utilities|FlowControl|Gate true
    (:Exit
      (|CallParentFunction)
      (Variables|Default|SetReleased? false)
      (if (Variables|Default|GetCanFire?)
        (Variables|Default|SetCanFire? false)
        (if (not (Variables|Default|GetReleased?))
          (if (> (Variables|Default|GetPistolAmmo) 0)
            (bind _returnvalue (Game|SpawnActorfromClass "/Game/Blueprints/WeaponBP/SMG_Proj.SMG_Proj_C" (Variables|Default|GetProjectileHit) "AdjustIfPossibleButDontSpawnIfColliding" 0 "0.000000,0.000000,0.000000" 0)) ; Spawn projectile
            (Utilities|Array|Add (Variables|Default|GetSavedProjectile) _returnvalue)
            (bind _output_get (Variables|Default|SetPistolAmmo (- (Variables|Default|GetPistolAmmo) 1)))
            (CallFunction|UpdateAmmo _output_get)
            (if (> (Variables|Default|GetPistolAmmo) 0)
              (Utilities|Time|SetTimerbyFunctionName 0 "ShotTimerExpired" (Variables|Default|GetPistolFireRate))
              (Audio|PlaySoundatLocation "/Game/ArtAssets/Audio/FirstPersonTemplateWeaponFire02.FirstPersonTemplateWeaponFire02" (Transformation|GetActorLocation)) ; Play firing sound
              (else
                (Utilities|Time|SetTimerbyFunctionName 0 "ShotTimerExpired" (Variables|Default|GetPistolReloadTime))
                (Variables|Default|SetPistolAmmo (Variables|Default|GetMaxPistolAmmo))))))))))

(event EventFireMain
  (Utilities|FlowControl|Gate true) ; enters at Open
)

(event EventMainRelease
  (Variables|Default|SetReleased? true)
  (Variables|Default|SetCanFire? true)
  (Utilities|FlowControl|Sequence
    (:then_0
      (Utilities|FlowControl|Gate true) ; enters at Close
    )
    (:then_1
      (Utilities|FlowControl|Delay 0.4)
      (if (== (Utilities|Array|Length (Variables|Default|GetSavedProjectile)) 0) :!label _label
        (Variables|Default|SetMagnumIndex 0)
        (else
          (bind _assmg_proj (Utilities|Casting|CastToSMG_Proj (Utilities|Array|Get(acopy) (Variables|Default|GetSavedProjectile) (Variables|Default|GetMagnumIndex))))
          (Default|Detonate _assmg_proj)
          (Variables|Default|SetMagnumIndex (+ (Variables|Default|GetMagnumIndex) 1))
          (Utilities|FlowControl|Delay 0.1)
          (goto _label))))))

(fn ConstructionScript
  (|CallParentFunction))