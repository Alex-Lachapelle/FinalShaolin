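; Rain weapon Blueprint that spawns a RainCloud actor where the shot hits.
; On FireMain it runs the parent fire logic, then places the cloud 200 units out from the HitResult impact point along the surface normal, with no rotation.
; The spawned cloud is stored in a variable, and no other events add logic beyond parent calls.
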(event EventBeginPlay
  (|CallParentFunction))

(event EventActorBeginOverlap
  (params (OtherActor :type Actor%20Object%20Reference)))

(event EventTick
  (params (DeltaSeconds :type Float%20%28single-precision%29))
  (|CallParentFunction 0.0))

(event EventFireMain
  (bind _hitresult (Variables|Default|GetHitResult))
  (bind (_bblockinghit _binitialoverlap _time _location _impactpoint _normal _impactnormal) (Collision|BreakHitResult _hitresult))
  (|CallParentFunction)
  (bind _returnvalue (Game|SpawnActorfromClass "/Game/Blueprints/WeaponBP/RainCloud.RainCloud_C" (Math|Transform|MakeTransform (+ _impactpoint (* _impactnormal 2e+02))) "Undefined" 0 0))
  (Variables|Default|SetNewVar_0_0 _returnvalue))

(fn ConstructionScript
  (|CallParentFunction))