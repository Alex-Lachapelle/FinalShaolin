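; LaserDisc is a charge-and-release weapon that fires a LaserDisc_Proj disc from the player's gun.
; FireMain starts charging, and Tick raises ChargeTime up to a cap.
; MainRelease line-traces from the first-person camera, then spawns the projectile at the gun, aimed at the impact or max-range point.
; Charge time sets projectile scale and multiplier, then resets as the ShotTimerExpired timer starts.
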(event EventFireMain
  (Variables|Default|SetCharging? true)
  (if (Variables|Default|GetCanFire?)
    (Variables|Default|SetCanFire? false)))

(event EventMainRelease
  (bind _asfirst_person_character (Utilities|Casting|CastToFirstPersonCharacter (Game|Player|GetPlayerPawn 0)))
  (Variables|Default|SetMaxRangeHitPoint (+ (Transformation|GetWorldLocation (Variables|/Game/Blueprints/Player/FirstPersonCharacter.FirstPersonCharacter_C|GetFirstPersonCamera _asfirst_person_character)) (* (Math|Vector|GetForwardVector (Transformation|GetWorldRotation (Variables|/Game/Blueprints/Player/FirstPersonCharacter.FirstPersonCharacter_C|GetFirstPersonCamera _asfirst_person_character))) (Variables|Default|GetMaxRange))))
  (bind (_outhit _returnvalue) (Collision|LineTraceByChannel (Transformation|GetWorldLocation (Variables|/Game/Blueprints/Player/FirstPersonCharacter.FirstPersonCharacter_C|GetFirstPersonCamera _asfirst_person_character)) (+ (Transformation|GetWorldLocation (Variables|/Game/Blueprints/Player/FirstPersonCharacter.FirstPersonCharacter_C|GetFirstPersonCamera _asfirst_person_character)) (* (Math|Vector|GetForwardVector (Transformation|GetWorldRotation (Variables|/Game/Blueprints/Player/FirstPersonCharacter.FirstPersonCharacter_C|GetFirstPersonCamera _asfirst_person_character))) (Variables|Default|GetMaxRange))) "TraceTypeQuery1" false 0 "None"))
  (bind _asfirst_person_character_2 (Utilities|Casting|CastToFirstPersonCharacter (Game|Player|GetPlayerPawn 0))
    (:then
      _)
    (:CastFailed
      _))
  (if _returnvalue
    (Variables|Default|SetDiscProjectileHit (Math|Transform|MakeTransform (.Location (Math|Transform|BreakTransform (Variables|/Game/Blueprints/Player/FirstPersonCharacter.FirstPersonCharacter_C|GetGunTransform _asfirst_person_character_2))) (Math|Rotator|MakeRotfromX (- (.ImpactPoint (Collision|BreakHitResult _outhit)) (.Location (Math|Transform|BreakTransform (Variables|/Game/Blueprints/Player/FirstPersonCharacter.FirstPersonCharacter_C|GetGunTransform _asfirst_person_character_2)))))))
    (else
      (Variables|Default|SetDiscProjectileHit (Math|Transform|MakeTransform (.Location (Math|Transform|BreakTransform (Variables|/Game/Blueprints/Player/FirstPersonCharacter.FirstPersonCharacter_C|GetGunTransform _asfirst_person_character_2))) (Math|Rotator|MakeRotfromX (- (Variables|Default|GetMaxRangeHitPoint) (.Location (Math|Transform|BreakTransform (Variables|/Game/Blueprints/Player/FirstPersonCharacter.FirstPersonCharacter_C|GetGunTransform _asfirst_person_character_2)))))))))
  (Game|SpawnActorfromClass "/Game/Blueprints/WeaponBP/LaserDisc_Proj.LaserDisc_Proj_C" (Variables|Default|GetDiscProjectileHit) "AdjustIfPossibleButDontSpawnIfColliding" 0 (* "0.040000,1.000000,0.030000" (Variables|Default|GetChargeTime)) (Variables|Default|GetChargeTime)) ; Spawn projectile
  (Variables|Default|SetCharging? false)
  (Variables|Default|SetCharged? false)
  (Variables|Default|SetChargeTime 0.0)
  (Utilities|Time|SetTimerbyFunctionName 0 "ShotTimerExpired" 0.1))

(event EventBeginPlay
  (|CallParentFunction))

(event EventActorBeginOverlap
  (params (OtherActor :type Actor%20Object%20Reference)))

(event EventTick
  (params (DeltaSeconds :type Float%20%28single-precision%29))
  (if (Variables|Default|GetCharging?)
    (if (not (>= (+ (* DeltaSeconds 2.0) (Variables|Default|GetChargeTime)) 4.0))
      (Variables|Default|SetChargeTime (+ (* DeltaSeconds 2.0) (Variables|Default|GetChargeTime)))
      (Variables|Default|SetCharged? true))))

(fn ConstructionScript
  (|CallParentFunction))