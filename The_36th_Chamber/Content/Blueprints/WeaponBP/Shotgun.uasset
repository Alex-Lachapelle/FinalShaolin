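; Shotgun weapon, a child Blueprint that fires a patterned burst of Shotgun_Proj projectiles on main fire.
; FireMain, gated by CanFire, spawns a center shot at ProjectileHit plus two rings of half BulletAmount each, at full and half Spread, then starts the Firerate timer for ShotTimerExpired.
; Transform spaces ring shots evenly around the aim axis using sine and cosine.
; FireAlt only calls the parent's FireMain.
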(event EventBeginPlay
  (|CallParentFunction))

(event EventActorBeginOverlap
  (params (OtherActor :type Actor%20Object%20Reference)))

(event EventFireMain
  (bind _bulletamount (Variables|Default|GetBulletAmount))
  (bind _bulletamount_2 (Variables|Default|GetBulletAmount))
  (bind _returnvalue (/ _bulletamount 2))
  (bind _returnvalue_2 (/ _bulletamount_2 2))
  (|CallParentFunction)
  (if (Variables|Default|GetCanFire?)
    (Variables|Default|SetCanFire? false)
    ;[1 1 1] Initial Projectile
    (Game|SpawnActorfromClass "/Game/Blueprints/WeaponBP/Shotgun_Proj.Shotgun_Proj_C" (Variables|Default|GetProjectileHit) "AdjustIfPossibleButDontSpawnIfColliding" 0 "0.000000,0.000000,0.000000" 0) ; Spawn projectile
    (Utilities|Time|SetTimerbyFunctionName 0 "ShotTimerExpired" (Variables|Default|GetFirerate))
    ;[1 1 1] Outer Radius
    (for _index (range 1 _returnvalue_2)
      (Game|SpawnActorfromClass "/Game/Blueprints/WeaponBP/Shotgun_Proj.Shotgun_Proj_C" (Utilities|Transform (Variables|Default|GetSpread) _index _returnvalue_2) "AdjustIfPossibleButDontSpawnIfColliding" 0 "0.000000,0.000000,0.000000" 0) ; Spawn projectile
    )
    ;[1 1 1] Inner Radius
    (for _index_2 (range 1 _returnvalue)
      (Game|SpawnActorfromClass "/Game/Blueprints/WeaponBP/Shotgun_Proj.Shotgun_Proj_C" (Utilities|Transform (/ (Variables|Default|GetSpread) 2.0) _index_2 _returnvalue) "AdjustIfPossibleButDontSpawnIfColliding" 0 "0.000000,0.000000,0.000000" 0) ; Spawn projectile
    )))

(event EventFireAlt
  (|CallParentFunction))

(fn ConstructionScript
  (|CallParentFunction))