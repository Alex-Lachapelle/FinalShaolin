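; MasterPawn is a character Blueprint, apparently a shared base, that handles damage and ragdoll death.
; AnyDamage lowers PawnHealth and briefly sets a Hit flag while slowing movement; a separate TakeDamage event lowers a different Health variable.
; Tick polls PawnHealth, then calls Death once, removes the capsule, ragdolls the mesh and destroys the actor after BodyLifetime.
; Projectile events store impact transform and velocity, which these graphs never read.
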(event Custom|ProjectileImpulse
  (params (Transform :type Transform) (Vector :type Vector))
  (Variables|Default|SetPhysicsTransform Transform)
  (Variables|Default|SetPhysicsVelocity Vector))

(event Custom|ProjectileLocation
  (params (Transform :type Transform))
  (Variables|Default|SetPhysicsTransform Transform))

(event Custom|TakeDamage
  (params (DamageTaken :type Integer))
  (Variables|Default|SetDamage DamageTaken)
  (Variables|Default|SetHealth (- (Variables|Default|GetHealth) (Variables|Default|GetDamage))))

(event Game|Damage|EventAnyDamage
  (params (Damage :type Float%20%28single-precision%29) (DamageType :type Damage%20Type%20Object%20Reference) (InstigatedBy :type Controller%20Object%20Reference) (DamageCauser :type Actor%20Object%20Reference))
  (Variables|Default|SetPawnDamage Damage)
  (Development|PrintString (Utilities|String|ToString(Float) Damage))
  (Variables|Default|SetPawnHealth (- (Variables|Default|GetPawnHealth) (Variables|Default|GetPawnDamage)))
  (Variables|Default|SetHit? true)
  (Variables|/Script/Engine.CharacterMovementComponent|SetMaxWalkSpeed (Variables|Character|GetCharacterMovement) 2e+01)
  (Utilities|FlowControl|Delay 0.125)
  (Variables|Default|SetHit? false)
  (Variables|/Script/Engine.CharacterMovementComponent|SetMaxWalkSpeed (Variables|Character|GetCharacterMovement) 8e+02))

(event EventBeginPlay)

(event EventActorBeginOverlap
  (params (OtherActor :type Actor%20Object%20Reference)))

(event EventTick
  (params (DeltaSeconds :type Float%20%28single-precision%29))
  (bind _mesh (Variables|Character|GetMesh))
  (if (<= (Variables|Default|GetPawnHealth) 0.0)
    (Utilities|FlowControl|Sequence
      (:then_0
        (Utilities|FlowControl|DoOnce false
          (:Completed
            (Default|CallDeath))))
      (:then_1
        (Variables|Default|SetDead? true)
        (Utilities|FlowControl|DoOnce false
          (:Completed
            (Components|DestroyComponent (Variables|Collision|GetCapsuleComponent))
            (Collision|SetCollisionEnabled _mesh "QueryAndPhysics")
            (Class|SkeletalMeshComponent|SetAllBodiesBelowSimulatePhysics _mesh (Class|SkinnedMeshComponent|GetBoneName _mesh 1) true)
            (Utilities|FlowControl|Delay (Variables|Default|GetBodyLifetime))
            (Actor|DestroyActor)))))))

(fn ConstructionScript)

(fn Physics)