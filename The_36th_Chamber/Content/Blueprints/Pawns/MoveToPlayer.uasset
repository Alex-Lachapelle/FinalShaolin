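; MoveToPlayer is a Behavior Tree task that moves the AI-controlled pawn to the actor stored in the TargetToFollow blackboard key.
; On execute it caches the owner as a BasicPawn_Controller, then runs AIMoveTo on that controller's pawn with a fixed acceptance radius.
; The task finishes successfully when the move succeeds, while a failed cast or move never calls FinishExecute.
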(event EventReceiveExecuteAI
  (params (OwnerController :type AI%20Controller%20Object%20Reference) (ControlledPawn :type Pawn%20Object%20Reference))
  (if (!= (Variables|Default|GetAiCon) 0)
    _
    (else
      (bind _asbasic_pawn_controller (Utilities|Casting|CastToBasicPawn_Controller OwnerController))
      (Variables|Default|SetAiCon _asbasic_pawn_controller)))
  (AI|AIMoveTo (Pawn|GetControlledPawn (Variables|Default|GetAiCon)) "0, 0, 0" (AI|BehaviorTree|GetBlackboardValueasActor (Variables|Default|GetTargetToFollow)) 1.2e+02 false
    (:OnSuccess
      (AI|BehaviorTree|FinishExecute true))))

(event EventReceiveExecute
  (params (OwnerActor :type Actor%20Object%20Reference))
  (if (!= (Variables|Default|GetAiCon) 0)
    _
    (else
      (bind _asbasic_pawn_controller (Utilities|Casting|CastToBasicPawn_Controller (stale EventReceiveExecuteAI OwnerController)))
      (Variables|Default|SetAiCon _asbasic_pawn_controller)))
  (AI|AIMoveTo (Pawn|GetControlledPawn (Variables|Default|GetAiCon)) "0, 0, 0" (AI|BehaviorTree|GetBlackboardValueasActor (Variables|Default|GetTargetToFollow)) 1.2e+02 false
    (:OnSuccess
      (AI|BehaviorTree|FinishExecute true))))