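; Behavior tree service that finds aggro targets for the pawn of a BasicPawn_Controller.
; Each tick it sphere-traces a very large radius for the desired object types, ignoring every MasterPawn.
; Each hit overwrites the TargetToFollow and TargetLocation blackboard keys, so the last one wins and nothing clears them.
; An unconnected variant holds a line-of-sight check that never runs.
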(event EventTick
  (params (OwnerActor :type Actor%20Object%20Reference) (DeltaSeconds :type Float%20%28single-precision%29))
  (if (!= (Variables|Default|GetBasicPawnCON_Ref) 0)
    _
    (else
      (bind _asbasic_pawn_controller (Utilities|Casting|CastToBasicPawn_Controller OwnerActor))
      (Variables|Default|SetBasicPawnCON_Ref _asbasic_pawn_controller)))
  (bind _outactors (Actor|GetAllActorsOfClass "/Game/Blueprints/Pawns/MasterPawn.MasterPawn_C"))
  (Variables|Default|SetMyLocation (Transformation|GetActorLocation (Pawn|GetControlledPawn (Variables|Default|GetBasicPawnCON_Ref))))
  (bind _outhits (Collision|MultiSphereTraceForObjects (Transformation|GetActorLocation (Pawn|GetControlledPawn (Variables|Default|GetBasicPawnCON_Ref))) (+ (Transformation|GetActorLocation (Pawn|GetControlledPawn (Variables|Default|GetBasicPawnCON_Ref))) "0, 0,15.000000") 1.55e+04 (Variables|Default|GetDesiredObjects) false _outactors "None"))
  (bind _array_element (Utilities|Array|ForEachLoopwithBreak _outhits)
    (:LoopBody
      (Class|BTFunctionLibrary|SetBlackboardValueasObject (Variables|Default|GetTargetToFollow) (.HitActor (Collision|BreakHitResult _array_element)))
      (AI|BehaviorTree|SetBlackboardValueasVector (Variables|Default|GetTargetLocation) (Transformation|GetActorLocation (.HitActor (Collision|BreakHitResult _array_element)))))))