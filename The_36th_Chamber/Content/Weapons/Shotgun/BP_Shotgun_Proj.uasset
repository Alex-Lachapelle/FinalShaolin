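; Shotgun projectile, built on a parent projectile class, whose damage depends on distance from the player.
; BeginPlay passes base damage to the parent and sets a short lifetime.
; On overlap, it divides damage by the overlapped actor's scaled distance from player pawn 0, runs parent overlap logic, then destroys itself.
; A hit on another object activates the impact effect and removes the trail, sphere and collision components.
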(event EventBeginPlay
  (CallFunction|SetDamage (Variables|Default|GetDamage))
  (|CallParentFunction)
  (Variables|Default|SetMaxLifetime 4.0)
  (Variables|Default|SetHitAnim? true))

(event EventActorBeginOverlap
  (params (OtherActor :type Actor%20Object%20Reference))
  (Variables|Default|SetHitLocation (Transformation|GetActorLocation OtherActor))
  (CallFunction|SetDamage (/ (Variables|Default|GetDamage) (/ (Math|Vector|VectorLength (- (Variables|Default|GetHitLocation) (Transformation|GetActorLocation (Game|Player|GetPlayerPawn 0)))) 6e+01)))
  (|CallParentFunction OtherActor)
  (Actor|DestroyActor))

(event EventTick
  (params (DeltaSeconds :type Float%20%28single-precision%29)))

(event Collision|EventHit
  (params (MyComp :type Primitive%20Component%20Object%20Reference) (Other :type Actor%20Object%20Reference) (OtherComp :type Primitive%20Component%20Object%20Reference) (bSelfMoved :type Boolean) (HitLocation :type Vector) (HitNormal :type Vector :default "0, 0, 0") (NormalImpulse :type Vector :default "0, 0, 0") (Hit :type Hit%20Result%20Structure%20%28by%20ref%29))
  (if (not (== Other self))
    (Components|Activation|Activate (Variables|Default|GetImpact) false)
    (Components|DestroyComponent (Variables|Default|GetTrail))
    (Components|DestroyComponent (Variables|Default|GetSphere))
    (Components|DestroyComponent (Variables|Default|GetCollisionComponent))))

(fn ConstructionScript
  (|CallParentFunction))