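; Shotgun weapon Blueprint whose main fire spawns a center pellet plus outer and inner rings of BP_Shotgun_Proj, each ring with randomized spread.
; The Transform helper holds trigonometry for spacing pellets evenly around the aim axis.
; A named timer paces shots; the last shell refills ammo immediately, starts the longer reload delay and skips the firing sound.
; Switching also refills ammo, and alt fire only makes a parent call.
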(event EventSwitching
  (bind _output_get (Variables|Default|SetShotgunAmmo (Variables|Default|GetMaxShotgunAmmo)))
  (CallFunction|UpdateAmmo _output_get))

(event EventBeginPlay
  (bind _output_get (Variables|Default|SetShotgunAmmo (Variables|Default|GetMaxShotgunAmmo)))
  (CallFunction|UpdateAmmo _output_get))

(event EventActorBeginOverlap
  (params (OtherActor :type Actor%20Object%20Reference)))

(event EventFireMain
  (bind _bulletcount (Variables|Default|GetBulletCount))
  (bind _bulletcount_2 (Variables|Default|GetBulletCount))
  (bind _returnvalue (/ _bulletcount 2))
  (bind _returnvalue_2 (/ _bulletcount_2 2))
  (|CallParentFunction)
  (if (Variables|Default|GetCanFire?)
    (Variables|Default|SetCanFire? false)
    (if (> (Variables|Default|GetShotgunAmmo) 0)
      ;[1 1 1] Initial Projectile
      (Game|SpawnActorfromClass "/Game/Weapons/Shotgun/BP_Shotgun_Proj.BP_Shotgun_Proj_C" (Variables|Default|GetProjectileHit) "AdjustIfPossibleButDontSpawnIfColliding" 0 (Variables|Default|GetCenterProjectileDamage) "0.000000,0.000000,0.000000") ; Spawn projectile
      (Utilities|Time|SetTimerbyFunctionName 0 "ShotTimerExpired" (Variables|Default|GetFirerate))
      ;[1 1 1] Outer Radius
      (for _index (range 1 _returnvalue_2)
        (Game|SpawnActorfromClass "/Game/Weapons/Shotgun/BP_Shotgun_Proj.BP_Shotgun_Proj_C" (Utilities|Transform (Math|Random|RandomFloatinRange 0.07 0.12) _index _returnvalue_2) "AdjustIfPossibleButDontSpawnIfColliding" 0 6e+02 "0.000000,0.000000,0.000000") ; Spawn projectile
      )
      ;[1 1 1] Inner Radius
      (for _index_2 (range 1 _returnvalue)
        (Game|SpawnActorfromClass "/Game/Weapons/Shotgun/BP_Shotgun_Proj.BP_Shotgun_Proj_C" (Utilities|Transform (Math|Random|RandomFloatinRange 0.03 0.07) _index_2 _returnvalue) "AdjustIfPossibleButDontSpawnIfColliding" 0 6e+02 "0.000000,0.000000,0.000000") ; Spawn projectile
      )
      (bind _output_get (Variables|Default|SetShotgunAmmo (- (Variables|Default|GetShotgunAmmo) 1)))
      (CallFunction|UpdateAmmo _output_get)
      (if (> (Variables|Default|GetShotgunAmmo) 0)
        (Utilities|Time|SetTimerbyFunctionName 0 "ShotTimerExpired" (Variables|Default|GetFirerate))
        (Audio|PlaySoundatLocation "/Game/Audio/FirstPersonTemplateWeaponFire02.FirstPersonTemplateWeaponFire02" (Transformation|GetActorLocation)) ; Play firing sound
        (else
          (Utilities|Time|SetTimerbyFunctionName 0 "ShotTimerExpired" (Variables|Default|GetShotgunReloadTime))
          (bind _output_get_2 (Variables|Default|SetShotgunAmmo (Variables|Default|GetMaxShotgunAmmo)))
          (CallFunction|UpdateAmmo _output_get_2))))))

(event EventFireAlt
  (|CallParentFunction))

(fn ConstructionScript
  (|CallParentFunction))