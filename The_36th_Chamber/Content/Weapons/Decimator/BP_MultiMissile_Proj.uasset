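; Homing missile projectile for the Decimator weapon that steers toward the impact point of its parent gun's hit result.
; BeginPlay sets damage, launches it forward with the player's velocity added, and opens the steering gate.
; Each Tick reads and debug-prints that impact point, then turns the missile toward it and sweeps it forward by a fixed per-frame step, independent of delta time.
; Hit and overlap handling defer to the parent class.
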(event OnComponentBeginOverlap(CollisionComponent)
  (params (OtherActor :type Actor%20Object%20Reference) (OtherComp :type Primitive%20Component%20Object%20Reference) (OtherBodyIndex :type Integer) (bFromSweep :type Boolean) (SweepResult :type Hit%20Result%20Structure%20%28by%20ref%29)))

(event Collision|EventActorBeginOverlap
  (params (OtherActor :type Actor%20Object%20Reference))
  (|CallParentFunction OtherActor))

(event Collision|EventHit
  (params (MyComp :type Primitive%20Component%20Object%20Reference) (Other :type Actor%20Object%20Reference) (OtherComp :type Primitive%20Component%20Object%20Reference) (bSelfMoved :type Boolean) (HitLocation :type Vector) (HitNormal :type Vector) (NormalImpulse :type Vector) (Hit :type Hit%20Result%20Structure%20%28by%20ref%29))
  (|CallParentFunction MyComp Other OtherComp bSelfMoved HitLocation HitNormal NormalImpulse Hit))

(event EventBeginPlay
  (CallFunction|SetDamage (Variables|Default|GetDamage))
  (bind _asfirst_person_character (Utilities|Casting|CastToFirstPersonCharacter (Game|GetPlayerCharacter 0)))
  (Game|Components|ProjectileMovement|SetVelocityinLocalSpace (Variables|Default|GetProjectile) (+ (Math|Vector|UnrotateVector (Transformation|GetVelocity _asfirst_person_character) (Pawn|GetControlRotation _asfirst_person_character :!class /Script/Engine.Pawn)) "5000.000000, 0, 0"))
  (Utilities|FlowControl|Gate true) ; enters at Open
)

(event EventActorBeginOverlap
  (params (OtherActor :type Actor%20Object%20Reference)))

(event EventTick
  (params (DeltaSeconds :type Float%20%28single-precision%29))
  (Utilities|FlowControl|Sequence
    (:then_0
      (bind _asmaster_gun (Utilities|Casting|CastToMaster_Gun (Variables|Default|GetParentGun)))
      (bind _output_get (Variables|Default|SetLoc (.ImpactPoint (Collision|BreakHitResult (Variables|/Game/Weapons/Master_Gun.Master_Gun_C|GetHitResult _asmaster_gun)))))
      (Development|PrintString (Utilities|String|ToString(Vector) _output_get)))
    (:then_1
      (Utilities|FlowControl|Gate true
        (:Exit
          (Transformation|SetActorRotation (Math|Rotator|FindLookatRotation (Transformation|GetActorLocation) (Variables|Default|GetLoc)))
          (Transformation|SetActorRelativeLocation (+ (* (Math|Vector|GetForwardVector (Transformation|GetActorRotation)) 45.0) (Transformation|GetActorLocation)) true))))))

(fn ConstructionScript
  (|CallParentFunction))