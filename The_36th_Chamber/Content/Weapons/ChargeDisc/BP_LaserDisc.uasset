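; BP_LaserDisc is a charge weapon that fires a laser disc projectile on release.
; FireMain starts charging and Tick builds ChargeTime while it stays below a cap.
; MainRelease traces from the first-person camera and aims the muzzle spawn at the hit point or max range.
; ChargeTime sets the projectile's scale and charge multiplier, then resets as a short shot timer starts.
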(event EventFireMain
  (Variables|Default|SetCharging? true)
  (if (Variables|Default|GetCanFire?)
    (Variables|Default|SetCanFire? false)))

(event EventMainRelease
  (bind _guntransform (Variables|Default|GetGunTransform))
  (bind _location (Math|Transform|BreakTransform _guntransform))
  (bind _asfirst_person_character (Utilities|Casting|CastToFirstPersonCharacter (Game|Player|GetPlayerPawn 0)))
  (Variables|Default|SetMaxRangeHitPoint (+ (Transformation|GetWorldLocation (Variables|/Game/Character/FirstPersonCharacter.FirstPersonCharacter_C|GetFirstPersonCamera _asfirst_person_character)) (* (Math|Vector|GetForwardVector (Transformation|GetWorldRotation (Variables|/Game/Character/FirstPersonCharacter.FirstPersonCharacter_C|GetFirstPersonCamera _asfirst_person_character))) (Variables|Default|GetMaxRange))))
  (bind (_outhit _returnvalue) (Collision|LineTraceByChannel (Transformation|GetWorldLocation (Variables|/Game/Character/FirstPersonCharacter.FirstPersonCharacter_C|GetFirstPersonCamera _asfirst_person_character)) (+ (Transformation|GetWorldLocation (Variables|/Game/Character/FirstPersonCharacter.FirstPersonCharacter_C|GetFirstPersonCamera _asfirst_person_character)) (* (Math|Vector|GetForwardVector (Transformation|GetWorldRotation (Variables|/Game/Character/FirstPersonCharacter.FirstPersonCharacter_C|GetFirstPersonCamera _asfirst_person_character))) (Variables|Default|GetMaxRange))) "TraceTypeQuery1" false 0 "None"))
  (CallFunction|GetMuzzle)
  (if _returnvalue
    (Variables|Default|SetDiscProjectileHit (Math|Transform|MakeTransform _location (Math|Rotator|MakeRotfromX (- (.ImpactPoint (Collision|BreakHitResult _outhit)) _location))))
    (else
      (Variables|Default|SetDiscProjectileHit (Math|Transform|MakeTransform _location (Math|Rotator|MakeRotfromX (- (Variables|Default|GetMaxRangeHitPoint) _location))))))
  (Game|SpawnActorfromClass "/Game/Weapons/ChargeDisc/BP_LaserDisc_Proj.BP_LaserDisc_Proj_C" (Variables|Default|GetDiscProjectileHit) "AdjustIfPossibleButDontSpawnIfColliding" 0 (* "0.040000,1.000000,0.030000" (Variables|Default|GetChargeTime)) (Variables|Default|GetChargeTime)) ; Spawn projectile
  (Variables|Default|SetCharging? false)
  (Variables|Default|SetCharged? false)
  (Variables|Default|SetChargeTime 0.0)
  (Utilities|Time|SetTimerbyFunctionName 0 "ShotTimerExpired" 0.1))

(event EventBeginPlay
  (|CallParentFunction))

(event EventActorBeginOverlap
  (params (OtherActor :type Actor%20Object%20Reference)))

(event EventTick
  (params (DeltaSeconds :type Float%20%28single-precision%29))
  (if (Variables|Default|GetCharging?)
    (if (not (>= (+ (* DeltaSeconds 2.0) (Variables|Default|GetChargeTime)) 4.0))
      (Variables|Default|SetChargeTime (+ (* DeltaSeconds 2.0) (Variables|Default|GetChargeTime)))
      (Variables|Default|SetCharged? true))))

(fn ConstructionScript
  (|CallParentFunction))