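; BP_Crossbow2 is a crossbow weapon, derived from a parent gun class, that fires a bolt projectile.
; FireMain runs the parent logic, then, if CanFire is set, clears that flag, spawns a BP_Crossbow_Proj and stops firing.
; The projectile spawns at the ProjectileHit transform and receives a small scale and the bone name from the hit result.
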(event EventFireMain
  (|CallParentFunction)
  (if (Variables|Default|GetCanFire?)
    (Variables|Default|SetCanFire? false)
    (Game|SpawnActorfromClass "/Game/Weapons/Crossbow/BP_Crossbow_Proj.BP_Crossbow_Proj_C" (Variables|Default|GetProjectileHit) "AdjustIfPossibleButDontSpawnIfColliding" 0 "0.100000,0.100000,0.100000" (.HitBoneName (Collision|BreakHitResult (Variables|Default|GetHitResult)))) ; Spawn projectile
    (CallFunction|StopFiring)))

(event EventBeginPlay
  (|CallParentFunction))

(event EventActorBeginOverlap
  (params (OtherActor :type Actor%20Object%20Reference)))

(event EventTick
  (params (DeltaSeconds :type Float%20%28single-precision%29)))

(fn ConstructionScript
  (|CallParentFunction))