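; BP_Boomstick is a shotgun weapon that fires a single multi-projectile blast through an override of FireMain.
; When CanFire is set, it clears the flag, spawns a high-damage center projectile and calls StopFiring.
; It then spawns two half-BulletAmount pellet groups, outer and inner, with random spread per pellet.
; Transform supplies pellet placement, though its trigonometric ring-offset nodes appear unconnected here.
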(event EventBeginPlay)

(event EventActorBeginOverlap
  (params (OtherActor :type Actor%20Object%20Reference)))

(event EventTick
  (params (DeltaSeconds :type Float%20%28single-precision%29)))

(event EventFireMain
  (bind _bulletamount (Variables|Default|GetBulletAmount))
  (bind _bulletamount_2 (Variables|Default|GetBulletAmount))
  (bind _returnvalue (/ _bulletamount 2))
  (bind _returnvalue_2 (/ _bulletamount_2 2))
  (|CallParentFunction)
  (if (Variables|Default|GetCanFire?)
    (Variables|Default|SetCanFire? false)
    (Game|SpawnActorfromClass "/Game/Weapons/Shotgun/BP_Shotgun_Proj.BP_Shotgun_Proj_C" (Variables|Default|GetProjectileHit) "AdjustIfPossibleButDontSpawnIfColliding" 0 2e+03 "0.000000,0.000000,0.000000") ; Spawn projectile
    (CallFunction|StopFiring)
    (for _index (range 1 _returnvalue_2)
      (Game|SpawnActorfromClass "/Game/Weapons/Shotgun/BP_Shotgun_Proj.BP_Shotgun_Proj_C" (Utilities|Transform _index _returnvalue_2 (Math|Random|RandomFloatinRange 0.06 0.1)) "AdjustIfPossibleButDontSpawnIfColliding" 0 6e+02 "0.000000,0.000000,0.000000") ; Spawn projectile
    )
    (for _index_2 (range 1 _returnvalue)
      (Game|SpawnActorfromClass "/Game/Weapons/Shotgun/BP_Shotgun_Proj.BP_Shotgun_Proj_C" (Utilities|Transform _index_2 _returnvalue (Math|Random|RandomFloatinRange 0.03 0.06)) "AdjustIfPossibleButDontSpawnIfColliding" 0 6e+02 "0.000000,0.000000,0.000000") ; Spawn projectile
    )))

(fn ConstructionScript
  (|CallParentFunction))