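; BP_Magnum_Proj is the Magnum's explosive projectile, which attaches itself to any BP_MasterPawn it hits.
; Its Sphere1 blast volume has collision off from BeginPlay until a Detonate event, not called within this graph, enables it briefly before destroying the actor.
; Pawns overlapping the sphere take explosion damage credited to player 0's controller.
; The explosion emitter node is disconnected, so this graph spawns no effect.
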(event OnComponentBeginOverlap(Sphere1)
  (params (OtherActor :type Actor%20Object%20Reference) (OtherComp :type Primitive%20Component%20Object%20Reference) (OtherBodyIndex :type Integer) (bFromSweep :type Boolean) (SweepResult :type Hit%20Result%20Structure%20%28by%20ref%29))
  (bind _asbp_master_pawn (Utilities|Casting|CastToBP_MasterPawn OtherActor))
  (if (== _asbp_master_pawn OtherActor)
    (Game|Damage|ApplyDamage OtherActor (Variables|Default|GetExplosionDamage) (Game|GetPlayerController 0) self "/Game/Weapons/DmgType.DmgType_C")))

(event Custom|Detonate
  (Collision|SetCollisionEnabled (Variables|Default|GetSphere1) "QueryAndPhysics")
  (Utilities|FlowControl|Delay 0.2)
  (Actor|DestroyActor))

(event EventBeginPlay
  (Collision|SetCollisionEnabled (Variables|Default|GetSphere1) "NoCollision"))

(event EventActorBeginOverlap
  (params (OtherActor :type Actor%20Object%20Reference)))

(event EventTick
  (params (DeltaSeconds :type Float%20%28single-precision%29)))

(event Collision|EventHit
  (params (MyComp :type Primitive%20Component%20Object%20Reference) (Other :type Actor%20Object%20Reference) (OtherComp :type Primitive%20Component%20Object%20Reference) (bSelfMoved :type Boolean) (HitLocation :type Vector :default "0, 0, 0") (HitNormal :type Vector :default "0, 0, 0") (NormalImpulse :type Vector :default "0, 0, 0") (Hit :type Hit%20Result%20Structure%20%28by%20ref%29))
  (bind _asbp_master_pawn (Utilities|Casting|CastToBP_MasterPawn Other))
  (if (== _asbp_master_pawn Other)
    (Class|Actor|AttachRootComponentto OtherComp "None" "KeepWorldPosition" true)))

(fn ConstructionScript
  (|CallParentFunction))