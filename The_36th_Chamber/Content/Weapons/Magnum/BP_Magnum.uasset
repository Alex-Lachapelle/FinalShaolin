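; BP_Magnum is a magnum weapon that fires BP_Magnum_Proj projectiles with limited ammo, built on a parent weapon class.
; FireMain gates on CanFire, spawns and stores a projectile, decrements ammo and calls UpdateAmmo.
; A ShotTimerExpired timer uses the fire rate, or the reload time on the last round, which refills ammo immediately and plays no sound.
; BeginPlay fills ammo and calls Switching; FireAlt is empty.
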(event EventFireAlt)

(event EventBeginPlay
  (|CallParentFunction)
  (Variables|Default|SetPistolAmmo (Variables|Default|GetMaxPistolAmmo))
  (CallFunction|Switching))

(event EventActorBeginOverlap
  (params (OtherActor :type Actor%20Object%20Reference)))

(event EventTick
  (params (DeltaSeconds :type Float%20%28single-precision%29)))

(event EventFireMain
  (|CallParentFunction)
  (if (Variables|Default|GetCanFire?)
    (Variables|Default|SetCanFire? false)
    (if (> (Variables|Default|GetPistolAmmo) 0)
      (bind _returnvalue (Game|SpawnActorfromClass "/Game/Weapons/Magnum/BP_Magnum_Proj.BP_Magnum_Proj_C" (Variables|Default|GetProjectileHit) "AdjustIfPossibleButDontSpawnIfColliding" 0 "0.100000,0.100000,0.100000" 0)) ; Spawn projectile
      (Utilities|Array|Add (Variables|Default|GetSavedProjectile) _returnvalue)
      (bind _output_get (Variables|Default|SetPistolAmmo (- (Variables|Default|GetPistolAmmo) 1)))
      (CallFunction|UpdateAmmo _output_get)
      (if (> (Variables|Default|GetPistolAmmo) 0)
        (Utilities|Time|SetTimerbyFunctionName 0 "ShotTimerExpired" (Variables|Default|GetPistolFireRate))
        (Audio|PlaySoundatLocation "/Game/Audio/FirstPersonTemplateWeaponFire02.FirstPersonTemplateWeaponFire02" (Transformation|GetActorLocation)) ; Play firing sound
        (else
          (Utilities|Time|SetTimerbyFunctionName 0 "ShotTimerExpired" (Variables|Default|GetPistolReloadTime))
          (Variables|Default|SetPistolAmmo (Variables|Default|GetMaxPistolAmmo)))))))

(fn ConstructionScript
  (|CallParentFunction))