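; BP_Blizzard is a weapon Blueprint whose main fire spawns a rain cloud at the point it hits.
; FireMain runs the parent fire logic, then spawns BP_RainCloud offset from HitResult's impact point along the surface normal, with zero rotation and unit scale.
; It stores the new cloud in RainCloud and adds no other active logic of its own.
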(event EventBeginPlay
  (|CallParentFunction))

(event EventActorBeginOverlap
  (params (OtherActor :type Actor%20Object%20Reference)))

(event EventTick
  (params (DeltaSeconds :type Float%20%28single-precision%29)))

(event EventFireMain
  (bind _hitresult (Variables|Default|GetHitResult))
  (bind (_bblockinghit _binitialoverlap _time _location _impactpoint _normal _impactnormal) (Collision|BreakHitResult _hitresult))
  (|CallParentFunction)
  (bind _returnvalue (Game|SpawnActorfromClass "/Game/Weapons/Rain/BP_RainCloud.BP_RainCloud_C" (Math|Transform|MakeTransform (+ _impactpoint (* _impactnormal 2e+02))) "Undefined" 0 0))
  (Variables|Default|SetRainCloud _returnvalue))

(fn ConstructionScript
  (|CallParentFunction))