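; Crossbow weapon that fires projectiles and zooms the first-person player's view on alternate fire.
; FireMain runs the parent logic, spawns BP_Crossbow_Proj with a sound, decrements ammo and locks CanFire.
; A ShotTimerExpired timer follows at the fire-rate delay, or the longer-named reload delay when empty, where ammo refills at once without updating the display.
; Switching and BeginPlay refill ammo and update the display.
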(event EventSwitching
  (bind _output_get (Variables|Default|SetCrossbowAmmo (Variables|Default|GetMaxCrossbowAmmo)))
  (CallFunction|UpdateAmmo _output_get))

(event EventBeginPlay
  (|CallParentFunction)
  (Variables|Default|SetCrossbowAmmo (Variables|Default|GetMaxCrossbowAmmo))
  (CallFunction|Switching))

(event EventActorBeginOverlap
  (params (OtherActor :type Actor%20Object%20Reference)))

(event EventTick
  (params (DeltaSeconds :type Float%20%28single-precision%29))
  (|CallParentFunction 0.0))

(event EventFireMain
  (|CallParentFunction)
  (if (Variables|Default|GetCanFire?)
    (Variables|Default|SetCanFire? false)
    (Game|SpawnActorfromClass "/Game/Weapons/Crossbow/BP_Crossbow_Proj.BP_Crossbow_Proj_C" (Variables|Default|GetProjectileHit) "AdjustIfPossibleButDontSpawnIfColliding" 0 "0.100000,0.100000,0.100000" (.HitBoneName (Collision|BreakHitResult (Variables|Default|GetHitResult)))) ; Spawn projectile
    (Audio|PlaySoundatLocation "/Game/Audio/FirstPersonTemplateWeaponFire02.FirstPersonTemplateWeaponFire02" (Transformation|GetActorLocation)) ; Play firing sound
    (bind _output_get (Variables|Default|SetCrossbowAmmo (- (Variables|Default|GetCrossbowAmmo) 1)))
    (CallFunction|UpdateAmmo _output_get)
    (if (> (Variables|Default|GetCrossbowAmmo) 0)
      (Utilities|Time|SetTimerbyFunctionName 0 "ShotTimerExpired" (Variables|Default|GetCrossbowFirerate))
      (else
        (Utilities|Time|SetTimerbyFunctionName 0 "ShotTimerExpired" (Variables|Default|GetCrossbowReloadTime))
        (Variables|Default|SetCrossbowAmmo (Variables|Default|GetMaxCrossbowAmmo))))))

(event EventFireAlt
  (bind _asfirst_person_character (Utilities|Casting|CastToFirstPersonCharacter (Game|Player|GetPlayerPawn 0)))
  (Default|Zoom _asfirst_person_character))

(event EventAltRelease
  (bind _asfirst_person_character (Utilities|Casting|CastToFirstPersonCharacter (Game|Player|GetPlayerPawn 0)))
  (Default|UnZoom _asfirst_person_character))

(fn ConstructionScript
  (|CallParentFunction))