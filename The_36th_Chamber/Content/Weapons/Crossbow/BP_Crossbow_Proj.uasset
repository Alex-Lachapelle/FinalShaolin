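; Crossbow bolt projectile that damages the first MasterPawn it overlaps and pins itself to that pawn.
; On overlap, a DoN gate applies a fixed 5000 damage, stops physics simulation and joins the bolt to the pawn's mesh with a physics constraint.
; SetDamage stores a value the hit ignores, and the bone-name capture is disconnected.
; The projectile destroys itself 15 seconds after BeginPlay.
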(event OnComponentBeginOverlap(CollisionComponent)
  (params (OtherActor :type Actor%20Object%20Reference) (OtherComp :type Primitive%20Component%20Object%20Reference) (OtherBodyIndex :type Integer) (bFromSweep :type Boolean) (SweepResult :type Hit%20Result%20Structure%20%28by%20ref%29)))

(event Custom|SetDamage
  (params (SetDamage :type Float%20%28single-precision%29))
  (Variables|Default|SetProjectileDamage SetDamage))

(event EventBeginPlay
  (Utilities|FlowControl|Delay 15.0)
  (Actor|DestroyActor) ; Then destroy this projectile
)

(event Collision|EventActorBeginOverlap
  (params (OtherActor :type Actor%20Object%20Reference))
  (bind _asmaster_pawn (Utilities|Casting|CastToMasterPawn OtherActor))
  (if (== _asmaster_pawn OtherActor)
    (Utilities|FlowControl|DoN 1
      (:Exit
        (Variables|Default|SetHit? true)
        (Game|Damage|ApplyDamage OtherActor 5e+03 (Game|GetPlayerController 0) self "/Game/Weapons/DmgType.DmgType_C")
        (Physics|SetSimulatePhysics (Variables|MyProjectile|GetCollisionComponent) false)
        (Class|PhysicsConstraintComponent|SetConstrainedComponents (Variables|Default|GetPhysicsConstraint) (Variables|MyProjectile|GetCollisionComponent) "Grip" (Variables|/Script/Engine.Character|GetMesh _asmaster_pawn) (Variables|Default|GetBoneName))
        (Development|PrintString (Utilities|String|ToString(Name) "None"))))))

(event Collision|EventHit
  (params (MyComp :type Primitive%20Component%20Object%20Reference) (Other :type Actor%20Object%20Reference) (OtherComp :type Primitive%20Component%20Object%20Reference) (bSelfMoved :type Boolean) (HitLocation :type Vector) (HitNormal :type Vector :default "0, 0, 0") (NormalImpulse :type Vector :default "0, 0, 0") (Hit :type Hit%20Result%20Structure%20%28by%20ref%29)))

(event EventTick
  (params (DeltaSeconds :type Float%20%28single-precision%29)))

(fn ConstructionScript
  (Variables|Default|SetAlwaysDestroy? (Variables|Default|GetAlwaysDestroy?)))