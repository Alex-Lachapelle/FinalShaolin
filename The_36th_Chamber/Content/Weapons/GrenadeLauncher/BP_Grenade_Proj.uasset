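; BP_Grenade_Proj is the grenade launcher's projectile, a child Blueprint that explodes after bouncing.
; On BeginPlay it copies GrenadeDamage into ProjectileDamage, with the parent BeginPlay call left disabled.
; Each Hit event increments a bounce counter; on the third, it spawns an explosion particle effect at its location and destroys itself.
; The graph itself applies no damage on explosion.
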(event EventBeginPlay
  (Variables|Default|SetProjectileDamage (Variables|Default|GetGrenadeDamage)))

(event EventActorBeginOverlap
  (params (OtherActor :type Actor%20Object%20Reference))
  (|CallParentFunction 0))

(event EventTick
  (params (DeltaSeconds :type Float%20%28single-precision%29)))

(event Collision|EventHit
  (params (MyComp :type Primitive%20Component%20Object%20Reference) (Other :type Actor%20Object%20Reference) (OtherComp :type Primitive%20Component%20Object%20Reference) (bSelfMoved :type Boolean) (HitLocation :type Vector :default "0, 0, 0") (HitNormal :type Vector :default "0, 0, 0") (NormalImpulse :type Vector :default "0, 0, 0") (Hit :type Hit%20Result%20Structure%20%28by%20ref%29))
  (Variables|Default|SetBounces (+ (Variables|Default|GetBounces) 1))
  (if (== (Variables|Default|GetBounces) 3)
    (Effects|SpawnEmitteratLocation "/Game/Weapons/GrenadeLauncher/Assets/P_ExplosionBase.P_ExplosionBase" (Transformation|GetActorLocation))
    (Actor|DestroyActor)))

(fn ConstructionScript
  (|CallParentFunction))