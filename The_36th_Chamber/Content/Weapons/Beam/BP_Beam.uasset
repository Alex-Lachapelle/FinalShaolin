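; BP_Beam is a beam weapon that shows a continuous particle beam from the muzzle while fire is held.
; FireMain opens a Tick gate, and MainRelease closes it and deactivates the particle system.
; Each tick refreshes the muzzle transform, line traces 1500 units forward on Visibility, and sets the beam endpoints to the muzzle and the impact point or maximum range.
; The trace only positions the visual; no damage is applied here.
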(event EventBeginPlay
  (|CallParentFunction))

(event EventActorBeginOverlap
  (params (OtherActor :type Actor%20Object%20Reference)))

(event EventTick
  (params (DeltaSeconds :type Float%20%28single-precision%29))
  (bind _particlesystem_0 (Variables|Default|GetParticleSystem_0))
  (bind _guntransform (Variables|Default|GetGunTransform))
  (bind (_location _rotation) (Math|Transform|BreakTransform _guntransform))
  (bind _returnvalue (Math|Vector|GetForwardVector _rotation))
  (bind _returnvalue_2 (* _returnvalue 1.5e+03))
  (bind _returnvalue_3 (+ _location _returnvalue_2))
  (Utilities|FlowControl|Gate true
    (:Exit
      (Components|Activation|Activate (Variables|Default|GetParticleSystem_0) false)
      (CallFunction|GetMuzzle)
      (bind (_outhit _returnvalue_4) (Collision|LineTraceByChannel _location _returnvalue_3 "TraceTypeQuery1" true 0 "None"))
      (if (not (Variables|Default|GetCanFire?))
        (Class|ParticleSystemComponent|SetBeamSourcePoint _particlesystem_0 0 _location)
        (if _returnvalue_4
          (Class|ParticleSystemComponent|SetBeamTargetPoint _particlesystem_0 0 (.ImpactPoint (Collision|BreakHitResult _outhit)))
          (else
            (Class|ParticleSystemComponent|SetBeamTargetPoint _particlesystem_0 0 _returnvalue_3)))))))

(event EventFireMain
  (bind _particlesystem_0 (Variables|Default|GetParticleSystem_0))
  (bind _guntransform (Variables|Default|GetGunTransform))
  (bind (_location _rotation) (Math|Transform|BreakTransform _guntransform))
  (bind _returnvalue (Math|Vector|GetForwardVector _rotation))
  (bind _returnvalue_2 (* _returnvalue 1.5e+03))
  (bind _returnvalue_3 (+ _location _returnvalue_2))
  (if (Variables|Default|GetCanFire?)
    (Variables|Default|SetCanFire? false)
    (Utilities|FlowControl|Gate true) ; enters at Open
  ))

(event EventMainRelease
  (bind _particlesystem_0 (Variables|Default|GetParticleSystem_0))
  (bind _particlesystem_0_2 (Variables|Default|GetParticleSystem_0))
  (bind _guntransform (Variables|Default|GetGunTransform))
  (bind (_location _rotation) (Math|Transform|BreakTransform _guntransform))
  (bind _returnvalue (Math|Vector|GetForwardVector _rotation))
  (bind _returnvalue_2 (* _returnvalue 1.5e+03))
  (bind _returnvalue_3 (+ _location _returnvalue_2))
  (Variables|Default|SetCanFire? true)
  (Utilities|FlowControl|Sequence
    (:then_0
      (Utilities|FlowControl|Gate true) ; enters at Close
    )
    (:then_1
      (Components|Activation|Deactivate _particlesystem_0_2))))

(fn ConstructionScript
  (|CallParentFunction))