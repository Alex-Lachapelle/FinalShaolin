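; BP_EnergyBeam is a hold-to-fire weapon that shows a continuous beam from its muzzle while main fire is held.
; FireMain opens a Tick gate, and MainReleased closes it, resets CanFire and deactivates the particle system.
; Each gated tick traces forward on Visibility to a fixed range, placing the beam's endpoints at the muzzle and the impact point or maximum range.
; The beam applies no damage here, and alt fire is empty.
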(event EventMainReleased
  (bind _particlesystem (Variables|Default|GetParticleSystem))
  (bind _particlesystem_2 (Variables|Default|GetParticleSystem))
  (bind _muzzletransform (Variables|Default|GetMuzzleTransform))
  (bind (_location _rotation) (Math|Transform|BreakTransform _muzzletransform))
  (bind _returnvalue (Math|Vector|GetForwardVector _rotation))
  (bind _returnvalue_2 (* _returnvalue 1.5e+03))
  (bind _returnvalue_3 (+ _location _returnvalue_2))
  (Variables|Default|SetCanFire? true)
  (Utilities|FlowControl|Sequence
    (:then_0
      (Utilities|FlowControl|Gate true) ; enters at Close
    )
    (:then_1
      (Components|Activation|Deactivate _particlesystem))))

(event EventFireAlt)

(event EventFireMain
  (bind _particlesystem (Variables|Default|GetParticleSystem))
  (bind _muzzletransform (Variables|Default|GetMuzzleTransform))
  (bind (_location _rotation) (Math|Transform|BreakTransform _muzzletransform))
  (bind _returnvalue (Math|Vector|GetForwardVector _rotation))
  (bind _returnvalue_2 (* _returnvalue 1.5e+03))
  (bind _returnvalue_3 (+ _location _returnvalue_2))
  (if (Variables|Default|GetCanFire?)
    (Variables|Default|SetCanFire? false)
    (Utilities|FlowControl|Gate true) ; enters at Open
  ))

(event EventBeginPlay
  (|CallParentFunction))

(event EventActorBeginOverlap
  (params (OtherActor :type Actor%20Object%20Reference)))

(event EventTick
  (params (DeltaSeconds :type Float%20%28single-precision%29))
  (bind _particlesystem (Variables|Default|GetParticleSystem))
  (bind _muzzletransform (Variables|Default|GetMuzzleTransform))
  (bind (_location _rotation) (Math|Transform|BreakTransform _muzzletransform))
  (bind _returnvalue (Math|Vector|GetForwardVector _rotation))
  (bind _returnvalue_2 (* _returnvalue 1.5e+03))
  (bind _returnvalue_3 (+ _location _returnvalue_2))
  (Utilities|FlowControl|Gate true
    (:Exit
      (Components|Activation|Activate (Variables|Default|GetParticleSystem) false)
      (CallFunction|GetMuzzleTransform)
      (bind (_outhit _returnvalue_4) (Collision|LineTraceByChannel _location _returnvalue_3 "TraceTypeQuery1" true 0 "None"))
      (if (not (Variables|Default|GetCanFire?))
        (Class|ParticleSystemComponent|SetBeamSourcePoint _particlesystem 0 _location)
        (if _returnvalue_4
          (Class|ParticleSystemComponent|SetBeamTargetPoint _particlesystem 0 (.ImpactPoint (Collision|BreakHitResult _outhit)))
          (else
            (Class|ParticleSystemComponent|SetBeamTargetPoint _particlesystem 0 _returnvalue_3)))))))

(fn ConstructionScript
  (|CallParentFunction))