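; SMG weapon Blueprint that auto-fires projectiles while primary fire is held, then detonates them after release.
; Tick runs through a gate opened by FireMain, spawning and saving each projectile, with timers pacing shots and reloads.
; MainRelease closes the gate and, after a short delay, steps through the saved projectiles, detonating them in a staggered sequence.
; Ammo refills on empty, BeginPlay and weapon switch; alt fire is empty.
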(event EventFireAlt)

(event EventSwitching
  (params (Actor :type Actor%20Object%20Reference))
  (bind _output_get (Variables|Default|SetSMGAmmo (Variables|Default|GetMaxSMGAmmo)))
  (CallFunction|UpdateAmmo _output_get))

(event EventBeginPlay
  (|CallParentFunction)
  (bind _output_get (Variables|Default|SetSMGAmmo (Variables|Default|GetMaxSMGAmmo)))
  (CallFunction|UpdateAmmo _output_get))

(event Collision|EventActorBeginOverlap
  (params (OtherActor :type Actor%20Object%20Reference)))

(event EventTick
  (params (DeltaSeconds :type Float%20%28single-precision%29))
  (Utilities|FlowControl|Gate true
    (:Exit
      (|CallParentFunction)
      (Variables|Default|SetReleased? false)
      (if (Variables|Default|GetCanFire?)
        (Variables|Default|SetCanFire? false)
        (if (not (Variables|Default|GetReleased?))
          (if (> (Variables|Default|GetSMGAmmo) 0)
            (bind _returnvalue (Game|SpawnActorfromClass "/Game/Weapons/SMG/BP_SMG_Proj.BP_SMG_Proj_C" (Variables|Default|GetProjectileHit) "AdjustIfPossibleButDontSpawnIfColliding" 0 "0.000000,0.000000,0.000000" 0)) ; Spawn projectile
            (Utilities|Array|Add (Variables|Default|GetSavedProjectile) _returnvalue)
            (bind _output_get (Variables|Default|SetSMGAmmo (- (Variables|Default|GetSMGAmmo) 1)))
            (CallFunction|UpdateAmmo _output_get)
            (if (> (Variables|Default|GetSMGAmmo) 0)
              (Utilities|Time|SetTimerbyFunctionName 0 "ShotTimerExpired" (Variables|Default|GetSMGFireRate))
              (Audio|PlaySoundatLocation "/Game/Audio/FirstPersonTemplateWeaponFire02.FirstPersonTemplateWeaponFire02" (Transformation|GetActorLocation)) ; Play firing sound
              (else
                (Utilities|Time|SetTimerbyFunctionName 0 "ShotTimerExpired" (Variables|Default|GetSMGReloadTime))
                (bind _output_get_2 (Variables|Default|SetSMGAmmo (Variables|Default|GetMaxSMGAmmo)))
                (CallFunction|UpdateAmmo _output_get_2)))))))))

(event EventFireMain
  (Utilities|FlowControl|Gate true) ; enters at Open
)

(event EventMainRelease
  (Variables|Default|SetReleased? true)
  (Variables|Default|SetCanFire? true)
  (Utilities|FlowControl|Sequence
    (:then_0
      (Utilities|FlowControl|Gate true) ; enters at Close
    )
    (:then_1
      (Utilities|FlowControl|Delay 0.4)
      (if (== (Utilities|Array|Length (Variables|Default|GetSavedProjectile)) 0) :!label _label
        (Variables|Default|SetSMGIndex 0)
        (else
          (bind _asbp_smg_proj (Utilities|Casting|CastToBP_SMG_Proj (Utilities|Array|Get(acopy) (Variables|Default|GetSavedProjectile) (Variables|Default|GetSMGIndex))))
          (Default|Detonate _asbp_smg_proj)
          (Variables|Default|SetSMGIndex (+ (Variables|Default|GetSMGIndex) 1))
          (Utilities|FlowControl|Delay 0.1)
          (goto _label))))))

(fn ConstructionScript
  (|CallParentFunction))