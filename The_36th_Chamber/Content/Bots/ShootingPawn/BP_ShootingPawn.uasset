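; Bot pawn Blueprint that carries a skeletal gun on its mesh's GripPoint socket and fires projectiles on Shoot.
; Shoot passes through a gate, closed by StopShooting, and spawns a Master_PawnProjectile from the gun socket, crediting damage to the instigator's controller.
; A small random offset on the socket's forward vector adds one-sided spread.
; CanFire and the ShotTimer function enforce a cooldown between shots.
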(event Custom|Shoot
  (bind _gunsocket (Variables|Default|GetGunSocket))
  (bind _returnvalue (Transformation|GetWorldTransform _gunsocket))
  (bind (_location _rotation) (Math|Transform|BreakTransform _returnvalue))
  (bind (_x _y _z) (Math|Rotator|GetAxes _rotation))
  (Utilities|FlowControl|Sequence
    (:then_0
      (Utilities|FlowControl|Gate false :!label _label
        (:Exit
          (if (Variables|Default|GetCanFire?)
            (Game|SpawnActorfromClass "/Game/Bots/ShootingPawn/Weapons/Master_PawnProjectile.Master_PawnProjectile_C" (Math|Transform|MakeTransform _location (Math|Rotator|MakeRotfromX (+ (+ _x (* _y (Math|Random|RandomFloatinRange 0.0 0.02))) (* _z (Math|Random|RandomFloatinRange 0.0 0.02))))) "Undefined" 0 "0.000000,0.000000,0.000000" (Game|GetInstigatorController))
            (Variables|Default|SetCanFire? false)
            (Utilities|Time|SetTimerbyFunctionName 0 "ShotTimer" 1.0)))))
    (:then_1
      (goto _label Open))))

(event Custom|StopShooting
  (bind _gunsocket (Variables|Default|GetGunSocket))
  (bind _returnvalue (Transformation|GetWorldTransform _gunsocket))
  (bind (_location _rotation) (Math|Transform|BreakTransform _returnvalue))
  (bind (_x _y _z) (Math|Rotator|GetAxes _rotation))
  (Utilities|FlowControl|Gate false) ; enters at Close
)

(event EventBeginPlay)

(event EventActorBeginOverlap
  (params (OtherActor :type Actor%20Object%20Reference)))

(event EventTick
  (params (DeltaSeconds :type Float%20%28single-precision%29))
  (|CallParentFunction 0.0))

(fn ConstructionScript
  (|CallParentFunction)
  (Class|SceneComponent|Attachto (Variables|Default|GetSKGun) (Variables|Character|GetMesh) "GripPoint" "SnapToTargetIncludingScale" true))

(fn ShotTimer
  (Variables|Default|SetCanFire? true))