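; Suicide bot pawn that blows itself up, damaging itself and a nearby target.
; Explode waits briefly, then runs once to apply heavy self-damage and spawn an explosion emitter at its location.
; A single sphere trace around it, ignoring every BP_MasterPawn actor, applies the same damage to the one actor it hits.
; Both damage calls credit player controller 0 as instigator.
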(event Custom|Explode
  (bind _returnvalue (Transformation|GetActorLocation))
  (bind _self self)
  (Utilities|FlowControl|Delay 1.5)
  (Utilities|FlowControl|DoOnce false
    (:Completed
      (Game|Damage|ApplyDamage _self 2e+03 (Game|GetPlayerController 0) _self "/Game/Weapons/DmgType.DmgType_C")
      (Effects|SpawnEmitteratLocation "/Game/Weapons/GrenadeLauncher/Assets/P_ExplosionBase.P_ExplosionBase" (Transformation|GetActorLocation))
      (bind _outactors (Actor|GetAllActorsOfClass "/Game/Bots/BP_MasterPawn.BP_MasterPawn_C"))
      (bind (_outhit _returnvalue_2) (Collision|SphereTraceForObjects _returnvalue (+ _returnvalue "0, 0,15.000000") 5e+02 (Variables|Default|GetDesiredObjects) false _outactors "None"))
      (if _returnvalue_2
        (Game|Damage|ApplyDamage (.HitActor (Collision|BreakHitResult _outhit)) 2e+03 (Game|GetPlayerController 0) self "/Game/Weapons/DmgType.DmgType_C")))))

(event EventBeginPlay)

(event EventActorBeginOverlap
  (params (OtherActor :type Actor%20Object%20Reference)))

(event EventTick
  (params (DeltaSeconds :type Float%20%28single-precision%29))
  (|CallParentFunction 0.0))

(fn ConstructionScript
  (|CallParentFunction))