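; Base bot character that handles damage, hit reactions and ragdoll death.
; AnyDamage subtracts health and stores the damage causer's velocity, except crossbow bolts, which zero it and skip the hit reaction.
; Other projectiles flagged HitAnim briefly set Hit and slow walking.
; Tick polls health and, once depleted, fires CallDeath, ragdolls the mesh with half the stored velocity, removes the capsule and destroys the actor after BodyLifetime.
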(event Custom|CheckDeath)

(event Game|Damage|EventAnyDamage
  (params (Damage :type Float%20%28single-precision%29) (DamageType :type Damage%20Type%20Object%20Reference) (InstigatedBy :type Controller%20Object%20Reference) (DamageCauser :type Actor%20Object%20Reference))
  (Variables|Default|SetPhysicsVelocity (Transformation|GetVelocity DamageCauser))
  (Variables|Default|SetPawnDamage Damage)
  (Variables|Default|SetPawnHealth (- (Variables|Default|GetPawnHealth) (Variables|Default|GetPawnDamage)))
  (if (== DamageCauser "/Game/Weapons/Crossbow/BP_Crossbow_Proj.BP_Crossbow_Proj_C")
    (Variables|Default|SetPhysicsVelocity "0, 0, 0")
    (else
      (bind _asmaster_projectile (Utilities|Casting|CastToMaster_Projectile DamageCauser))
      (if (Variables|/Game/Weapons/Master_Projectile.Master_Projectile_C|GetHitAnim? _asmaster_projectile)
        (Variables|Default|SetHit? true)
        (Variables|/Script/Engine.CharacterMovementComponent|SetMaxWalkSpeed (Variables|Character|GetCharacterMovement) 2e+01)
        (Utilities|FlowControl|Delay 0.125)
        (Variables|Default|SetHit? false)
        (Variables|/Script/Engine.CharacterMovementComponent|SetMaxWalkSpeed (Variables|Character|GetCharacterMovement) 8e+02)))))

(event EventBeginPlay)

(event EventActorBeginOverlap
  (params (OtherActor :type Actor%20Object%20Reference)))

(event EventTick
  (params (DeltaSeconds :type Float%20%28single-precision%29))
  (bind _mesh (Variables|Character|GetMesh))
  (if (<= (Variables|Default|GetPawnHealth) 0.0)
    (Utilities|FlowControl|Sequence
      (:then_0
        (Utilities|FlowControl|DoOnce false
          (:Completed
            (Default|CallDeath))))
      (:then_1
        (Variables|Default|SetDead? true)
        (Utilities|FlowControl|DoOnce false
          (:Completed
            (Class|PrimitiveComponent|SetAllPhysicsLinearVelocity _mesh (/ (Variables|Default|GetPhysicsVelocity) 2.0) true)
            (Components|DestroyComponent (Variables|Collision|GetCapsuleComponent))
            (Collision|SetCollisionEnabled _mesh "PhysicsOnly")
            (Class|SkeletalMeshComponent|SetAllBodiesBelowSimulatePhysics _mesh (Class|SkinnedMeshComponent|GetBoneName _mesh 1) true)
            (Utilities|FlowControl|Delay (Variables|Default|GetBodyLifetime))
            (Actor|DestroyActor)))))))

(fn ConstructionScript)

(fn Physics)